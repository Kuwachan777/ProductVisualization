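; BPM_QuitSystem is a manager actor that quits the game when the end system widget signals it.
; On BeginPlay it finds the BPM_Widget actor, caches the WBPEndSystem from its widget, and binds its Quit event to that end system.
; Quit calls QuitGame for player controller 0, followed by a "Hello" debug print.
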(event Custom|Quit
  (Game|QuitGame (Game|GetPlayerController 0) "Quit" false)
  (Development|PrintString "Hello"))

(event EventBeginPlay
  (Utilities|FlowControl|Sequence
    (:then_0
      (bind _returnvalue (Actor|GetActorOfClass "/Game/Blueprint/Manager/BPM_Widget.BPM_Widget_C"))
      (Variables|Default|SetAsWBP_EndSystem (Variables|/Game/Blueprint/Widget/WBP_Widgets.WBP_Widgets_C|GetWBP_EndSystem (Variables|/Game/Blueprint/Manager/BPM_Widget.BPM_Widget_C|GetAsWBP_Widget _returnvalue))))
    (:then_1
      (EventDispatchers|BindEventtoEndSystem (Variables|Default|GetAsWBP_EndSystem) (delegate Custom|Quit)))))

(event Collision|EventActorBeginOverlap
  (params (OtherActor :type Actor%20Object%20Reference)))

(event EventTick
  (params (DeltaSeconds :type Float%20%28single-precision%29)))

(fn ConstructionScript)