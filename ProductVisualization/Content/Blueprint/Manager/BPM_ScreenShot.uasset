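; Screenshot manager actor that captures high-resolution screenshots at Full HD or 4K.
; On BeginPlay it finds the BPM_Widget manager in the level and caches its screenshot widget.
; It then binds that widget's Full HD and 4K events to handlers that run the HighResShot console command at the matching resolution.
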(event Custom|FullHDShot
  ;[1 1 1] Init Screen Shot
  (Development|ExecuteConsoleCommand "HighResShot 1920x1080" 0))

(event Custom|4KShot
  ;[1 1 1] Init Screen Shot
  (Development|ExecuteConsoleCommand "HighResShot 3840x2160" 0))

(event Custom|InitScreenShot
  (bind _wbp_screen_shot (Variables|Default|GetWBP%20Screen%20Shot))
  ;[1 1 1] Init Screen Shot
  (EventDispatchers|BindEventtoFullHDShot _wbp_screen_shot (delegate Custom|FullHDShot))
  (EventDispatchers|BindEventto4KShot _wbp_screen_shot (delegate Custom|4KShot)))

(event EventBeginPlay
  (Utilities|FlowControl|Sequence
    (:then_0
      (bind _returnvalue (Actor|GetActorOfClass "/Game/Blueprint/Manager/BPM_Widget.BPM_Widget_C"))
      (Variables|Default|SetWBP%20Screen%20Shot (Variables|/Game/Blueprint/Widget/WBP_Widgets.WBP_Widgets_C|GetWBP_ScreenShot (Variables|/Game/Blueprint/Manager/BPM_Widget.BPM_Widget_C|GetAsWBP_Widget _returnvalue))))
    (:then_1
      (CallFunction|InitScreenShot))))

(event Collision|EventActorBeginOverlap
  (params (OtherActor :type Actor%20Object%20Reference)))

(event EventTick
  (params (DeltaSeconds :type Float%20%28single-precision%29)))

(fn ConstructionScript)