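; Material manager that drives a runtime material editor for up to six meshes on the BP_Mesh actor.
; Mesh-select buttons choose the target and restore its saved slider values and enabled sliders.
; Preset buttons apply a new dynamic material instance and set which parameter sliders it allows.
; While the parameter window is shown, Tick pushes slider values into the selected instance and saves them per mesh.
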(event Custom|SetSliderEnable
  (params (SelectStruct :type Struct%20Enable%20Parameter%20Structure))
  (bind _aswbp_materialparameter (Variables|Default|GetAsWBP_MaterialParameter))
  ;[1 1 1] Init Meshes
  ;;[1 1 1] Set Parameter Slider Enable
  (Widget|SetIsEnabled (Variables|/Game/Blueprint/Widget/WBP_MaterialParameter.WBP_MaterialParameter_C|GetVB_TextureTiling _aswbp_materialparameter) (.texturetiling SelectStruct))
  (Widget|SetIsEnabled (Variables|/Game/Blueprint/Widget/WBP_MaterialParameter.WBP_MaterialParameter_C|GetVB_BaseColor _aswbp_materialparameter) (.basecolor SelectStruct))
  (Widget|SetIsEnabled (Variables|/Game/Blueprint/Widget/WBP_MaterialParameter.WBP_MaterialParameter_C|GetVB_Emissive _aswbp_materialparameter) (.emissive SelectStruct))
  (Widget|SetIsEnabled (Variables|/Game/Blueprint/Widget/WBP_MaterialParameter.WBP_MaterialParameter_C|GetVB_Metallic _aswbp_materialparameter) (.metallic SelectStruct))
  (Widget|SetIsEnabled (Variables|/Game/Blueprint/Widget/WBP_MaterialParameter.WBP_MaterialParameter_C|GetVB_Roughness _aswbp_materialparameter) (.roughtness SelectStruct))
  (Widget|SetIsEnabled (Variables|/Game/Blueprint/Widget/WBP_MaterialParameter.WBP_MaterialParameter_C|GetVB_Opacity _aswbp_materialparameter) (.opacity SelectStruct))
  (Widget|SetIsEnabled (Variables|/Game/Blueprint/Widget/WBP_MaterialParameter.WBP_MaterialParameter_C|GetVB_Refraction _aswbp_materialparameter) (.refraction SelectStruct))
  (Widget|SetIsEnabled (Variables|/Game/Blueprint/Widget/WBP_MaterialParameter.WBP_MaterialParameter_C|GetVB_Specular _aswbp_materialparameter) (.specular SelectStruct)))

(event Custom|SetMatDarkGreyFabric
  ;[1 1 1] Init Dynamic Material Instance
  ;;[1 1 1] Init Bind
  (bind _returnvalue (Rendering|Material|CreateDynamicMaterialInstance "/Game/Material/MI_Dark_Grey_Fabric_sbkla2p0_2K.MI_Dark_Grey_Fabric_sbkla2p0_2K" "None" "None" :!class /Script/Engine.KismetMaterialLibrary))
  (CallFunction|SetSelectDynamicMaterialInstance _returnvalue (Utilities|Struct|MakeStruct_EnableParameter true false false false false false false false)))

(event Custom|SetMatPatternedFabric
  ;[1 1 1] Init Dynamic Material Instance
  ;;[1 1 1] Init Bind
  (bind _returnvalue (Rendering|Material|CreateDynamicMaterialInstance "/Game/Material/MI_Patterned_Fabric_pcvg22p0_2K.MI_Patterned_Fabric_pcvg22p0_2K" "None" "None" :!class /Script/Engine.KismetMaterialLibrary))
  (CallFunction|SetSelectDynamicMaterialInstance _returnvalue (Utilities|Struct|MakeStruct_EnableParameter true false false false false false false false)))

(event Custom|SetMatWhiteCloth
  ;[1 1 1] Init Dynamic Material Instance
  ;;[1 1 1] Init Bind
  (bind _returnvalue (Rendering|Material|CreateDynamicMaterialInstance "/Game/Material/MI_White_Cloth_sbklx0p0_2K.MI_White_Cloth_sbklx0p0_2K" "None" "None" :!class /Script/Engine.KismetMaterialLibrary))
  (CallFunction|SetSelectDynamicMaterialInstance _returnvalue (Utilities|Struct|MakeStruct_EnableParameter true false false false false false false false)))

(event Custom|SetMatBrownLeather
  ;[1 1 1] Init Dynamic Material Instance
  ;;[1 1 1] Init Bind
  (bind _returnvalue (Rendering|Material|CreateDynamicMaterialInstance "/Game/Material/MI_Leather_oizuetp0_2K.MI_Leather_oizuetp0_2K" "None" "None" :!class /Script/Engine.KismetMaterialLibrary))
  (CallFunction|SetSelectDynamicMaterialInstance _returnvalue (Utilities|Struct|MakeStruct_EnableParameter true false false false false false false false)))

(event Custom|SetMatFabricLeather
  ;[1 1 1] Init Dynamic Material Instance
  ;;[1 1 1] Init Bind
  (bind _returnvalue (Rendering|Material|CreateDynamicMaterialInstance "/Game/Material/MI_Fabric_Leather_oizqhap0_2K.MI_Fabric_Leather_oizqhap0_2K" "None" "None" :!class /Script/Engine.KismetMaterialLibrary))
  (CallFunction|SetSelectDynamicMaterialInstance _returnvalue (Utilities|Struct|MakeStruct_EnableParameter true false false false false false false false)))

(event Custom|SetSelectDynamicMaterialInstance
  (params (SelectDynamicMaterialInstance :type Material%20Instance%20Dynamic%20Object%20Reference) (EnableParameter :type Struct%20Enable%20Parameter%20Structure))
  (bind _selectmesh (Variables|Default|GetSelectMesh))
  ;[1 1 1] Init Dynamic Material Instance
  (switch int (Variables|Default|GetSelectMeshNum)
    (:1
      (bind _output_get (Variables|Default|SetMash01SelectMaterial SelectDynamicMaterialInstance))
      (Rendering|Material|SetMaterial _selectmesh 0 _output_get)
      (bind _output_get_2 (Variables|Default|SetStructEnableSliderMesh01 EnableParameter))
      (CallFunction|SetSliderEnable _output_get_2))
    (:2
      (bind _output_get_3 (Variables|Default|SetMesh02SelectMaterial SelectDynamicMaterialInstance))
      (Rendering|Material|SetMaterial _selectmesh 0 _output_get_3)
      (bind _output_get_4 (Variables|Default|SetStructEnableSliderMesh02 EnableParameter))
      (CallFunction|SetSliderEnable _output_get_4))
    (:3
      (bind _output_get_5 (Variables|Default|SetMesh03SelectMaterial SelectDynamicMaterialInstance))
      (Rendering|Material|SetMaterial _selectmesh 0 _output_get_5)
      (bind _output_get_6 (Variables|Default|SetStructEnableSliderMesh03 EnableParameter))
      (CallFunction|SetSliderEnable _output_get_6))
    (:4
      (bind _output_get_7 (Variables|Default|SetMesh04SelectMaterial SelectDynamicMaterialInstance))
      (Rendering|Material|SetMaterial _selectmesh 0 _output_get_7)
      (bind _output_get_8 (Variables|Default|SetStructEnableSliderMesh04 EnableParameter))
      (CallFunction|SetSliderEnable _output_get_8))
    (:5
      (bind _output_get_9 (Variables|Default|SetMesh05SelectMaterial SelectDynamicMaterialInstance))
      (Rendering|Material|SetMaterial _selectmesh 0 _output_get_9)
      (bind _output_get_10 (Variables|Default|SetStructEnableSliderMesh05 EnableParameter))
      (CallFunction|SetSliderEnable _output_get_10))
    (:6
      (bind _output_get_11 (Variables|Default|SetMesh06SelectMaterial SelectDynamicMaterialInstance))
      (Rendering|Material|SetMaterial _selectmesh 0 _output_get_11)
      (bind _output_get_12 (Variables|Default|SetStructEnableSliderMesh06 EnableParameter))
      (CallFunction|SetSliderEnable _output_get_12))))

(event Custom|SetMatGypsum
  ;[1 1 1] Init Dynamic Material Instance
  ;;[1 1 1] Init Bind
  (bind _returnvalue (Rendering|Material|CreateDynamicMaterialInstance "/Game/Material/MI_Gypsum_Tiles_uldnbcdn_2K.MI_Gypsum_Tiles_uldnbcdn_2K" "None" "None" :!class /Script/Engine.KismetMaterialLibrary))
  (CallFunction|SetSelectDynamicMaterialInstance _returnvalue (Utilities|Struct|MakeStruct_EnableParameter true false false false false false false false)))

(event Custom|SetMatViaLatteaGranite
  ;[1 1 1] Init Dynamic Material Instance
  ;;[1 1 1] Init Bind
  (bind _returnvalue (Rendering|Material|CreateDynamicMaterialInstance "/Game/Material/MI_Via_Lattea_Granite_weoldhcv_2K.MI_Via_Lattea_Granite_weoldhcv_2K" "None" "None" :!class /Script/Engine.KismetMaterialLibrary))
  (CallFunction|SetSelectDynamicMaterialInstance _returnvalue (Utilities|Struct|MakeStruct_EnableParameter true false false false false false false false)))

(event Custom|SetMatDarkBrownLeather
  ;[1 1 1] Init Dynamic Material Instance
  ;;[1 1 1] Init Bind
  (bind _returnvalue (Rendering|Material|CreateDynamicMaterialInstance "/Game/Material/MI_Leather_sjqecg1c_2K.MI_Leather_sjqecg1c_2K" "None" "None" :!class /Script/Engine.KismetMaterialLibrary))
  (CallFunction|SetSelectDynamicMaterialInstance _returnvalue (Utilities|Struct|MakeStruct_EnableParameter true false false false false false false false)))

(event Custom|SetMatTranslucent
  ;[1 1 1] Init Dynamic Material Instance
  ;;[1 1 1] Init Bind
  (bind _returnvalue (Rendering|Material|CreateDynamicMaterialInstance "/Game/Material/MI_Translucent.MI_Translucent" "None" "None" :!class /Script/Engine.KismetMaterialLibrary))
  (CallFunction|SetSelectDynamicMaterialInstance _returnvalue (Utilities|Struct|MakeStruct_EnableParameter false true true false false true true false)))

(event Custom|SetMatDefaultWhite
  ;[1 1 1] Init Dynamic Material Instance
  ;;[1 1 1] Init Bind
  (bind _returnvalue (Rendering|Material|CreateDynamicMaterialInstance "/Game/Material/M_DefaultWhite.M_DefaultWhite" "None" "None" :!class /Script/Engine.KismetMaterialLibrary))
  (CallFunction|SetSelectDynamicMaterialInstance _returnvalue))

(event Custom|SetMatGlass
  ;[1 1 1] Init Dynamic Material Instance
  ;;[1 1 1] Init Bind
  (bind _returnvalue (Rendering|Material|CreateDynamicMaterialInstance "/Game/Material/MI_Glass.MI_Glass" "None" "None" :!class /Script/Engine.KismetMaterialLibrary))
  (CallFunction|SetSelectDynamicMaterialInstance _returnvalue (Utilities|Struct|MakeStruct_EnableParameter false true false false false false false false)))

(event Custom|SetMesh02
  ;[1 1 1] Init Meshes
  ;;[1 1 1] Set Select Mesh
  (Variables|Default|SetSelectMesh (Variables|/Game/Blueprint/Actor/BP_Mesh.BP_Mesh_C|GetStaticMesh02 (Variables|Default|GetAsBP_Mesh)))
  (Variables|Default|SetSelectMeshNum 2)
  (CallFunction|SetSliderValue (Variables|Default|GetStructParameterValueMesh02))
  (CallFunction|SetSliderEnable (Variables|Default|GetStructEnableSliderMesh02)))

(event Custom|SetMesh01
  ;[1 1 1] Init Meshes
  ;;[1 1 1] Set Select Mesh
  (Variables|Default|SetSelectMesh (Variables|/Game/Blueprint/Actor/BP_Mesh.BP_Mesh_C|GetStaticMesh01 (Variables|Default|GetAsBP_Mesh)))
  (Variables|Default|SetSelectMeshNum 1)
  (CallFunction|SetSliderValue (Variables|Default|GetStructParameterValueMesh01))
  (CallFunction|SetSliderEnable (Variables|Default|GetStructEnableSliderMesh01)))

(event Custom|SetMatMetallic
  ;[1 1 1] Init Dynamic Material Instance
  ;;[1 1 1] Init Bind
  (bind _returnvalue (Rendering|Material|CreateDynamicMaterialInstance "/Game/Material/MI_Metallic.MI_Metallic" "None" "None" :!class /Script/Engine.KismetMaterialLibrary))
  (CallFunction|SetSelectDynamicMaterialInstance _returnvalue (Utilities|Struct|MakeStruct_EnableParameter false true true false true false false true)))

(event Custom|SetMesh03
  ;[1 1 1] Init Meshes
  ;;[1 1 1] Set Select Mesh
  (Variables|Default|SetSelectMesh (Variables|/Game/Blueprint/Actor/BP_Mesh.BP_Mesh_C|GetStaticMesh03 (Variables|Default|GetAsBP_Mesh)))
  (Variables|Default|SetSelectMeshNum 3)
  (CallFunction|SetSliderValue (Variables|Default|GetStructParameterValueMesh03))
  (CallFunction|SetSliderEnable (Variables|Default|GetStructEnableSliderMesh03)))

(event Custom|SetMesh04
  ;[1 1 1] Init Meshes
  ;;[1 1 1] Set Select Mesh
  (Variables|Default|SetSelectMesh (Variables|/Game/Blueprint/Actor/BP_Mesh.BP_Mesh_C|GetStaticMesh04 (Variables|Default|GetAsBP_Mesh)))
  (Variables|Default|SetSelectMeshNum 4)
  (CallFunction|SetSliderValue (Variables|Default|GetStructParameterValueMesh04))
  (CallFunction|SetSliderEnable (Variables|Default|GetStructEnableSliderMesh04)))

(event Custom|SetMesh05
  ;[1 1 1] Init Meshes
  ;;[1 1 1] Set Select Mesh
  (Variables|Default|SetSelectMesh (Variables|/Game/Blueprint/Actor/BP_Mesh.BP_Mesh_C|GetStaticMesh05 (Variables|Default|GetAsBP_Mesh)))
  (Variables|Default|SetSelectMeshNum 5)
  (CallFunction|SetSliderValue (Variables|Default|GetStructParameterValueMesh05))
  (CallFunction|SetSliderEnable (Variables|Default|GetStructEnableSliderMesh05)))

(event Custom|SetMesh06
  ;[1 1 1] Init Meshes
  ;;[1 1 1] Set Select Mesh
  (Variables|Default|SetSelectMesh (Variables|/Game/Blueprint/Actor/BP_Mesh.BP_Mesh_C|GetStaticMesh06 (Variables|Default|GetAsBP_Mesh)))
  (Variables|Default|SetSelectMeshNum 6)
  (CallFunction|SetSliderValue (Variables|Default|GetStructParameterValueMesh06))
  (CallFunction|SetSliderEnable (Variables|Default|GetStructEnableSliderMesh06)))

(event Custom|SetStruct
  (params (BaseColorR :type Float%20%28double-precision%29) (BaseColorG :type Float%20%28double-precision%29) (BaseColorB :type Float%20%28double-precision%29) (Emissive :type Float%20%28double-precision%29) (Metallic :type Float%20%28double-precision%29) (Roughness :type Float%20%28double-precision%29) (TextureTiling :type Float%20%28double-precision%29) (Opacity :type Float%20%28double-precision%29) (Refraction :type Float%20%28double-precision%29) (Specular :type Float%20%28double-precision%29))
  ;[1 1 1] SetParameters
  (switch int (Variables|Default|GetSelectMeshNum)
    (:1
      (Variables|Default|SetStructParameterValueMesh01 (Utilities|Struct|MakeStruct_MaterialParameter BaseColorR BaseColorG BaseColorB Emissive Metallic Roughness TextureTiling Opacity Refraction Specular)))
    (:2
      (Variables|Default|SetStructParameterValueMesh02 (Utilities|Struct|MakeStruct_MaterialParameter BaseColorR BaseColorG BaseColorB Emissive Metallic Roughness TextureTiling Opacity Refraction Specular)))
    (:3
      (Variables|Default|SetStructParameterValueMesh03 (Utilities|Struct|MakeStruct_MaterialParameter BaseColorR BaseColorG BaseColorB Emissive Metallic Roughness TextureTiling Opacity Refraction Specular)))
    (:4
      (Variables|Default|SetStructParameterValueMesh04 (Utilities|Struct|MakeStruct_MaterialParameter BaseColorR BaseColorG BaseColorB Emissive Metallic Roughness TextureTiling Opacity Refraction Specular)))
    (:5
      (Variables|Default|SetStructParameterValueMesh05 (Utilities|Struct|MakeStruct_MaterialParameter BaseColorR BaseColorG BaseColorB Emissive Metallic Roughness TextureTiling Opacity Refraction Specular)))
    (:6
      (Variables|Default|SetStructParameterValueMesh06 (Utilities|Struct|MakeStruct_MaterialParameter BaseColorR BaseColorG BaseColorB Emissive Metallic Roughness TextureTiling Opacity Refraction Specular)))))

(event Custom|SetMatDefaultBlack
  ;[1 1 1] Init Dynamic Material Instance
  ;;[1 1 1] Init Bind
  (bind _returnvalue (Rendering|Material|CreateDynamicMaterialInstance "/Game/Material/M_DefaultBlack.M_DefaultBlack" "None" "None" :!class /Script/Engine.KismetMaterialLibrary))
  (CallFunction|SetSelectDynamicMaterialInstance _returnvalue))

(event Custom|InitBind
  ;[1 1 1] Init Dynamic Material Instance
  ;;[1 1 1] Init Bind
  (EventDispatchers|BindEventtoWhite (Variables|Default|GetAsWBP_MaterialParameter) (delegate Custom|SetMatDefaultWhite))
  (EventDispatchers|BindEventtoBlack (Variables|Default|GetAsWBP_MaterialParameter) (delegate Custom|SetMatDefaultBlack))
  (EventDispatchers|BindEventtoWood (Variables|Default|GetAsWBP_MaterialParameter) (delegate Custom|SetMatWood))
  (EventDispatchers|BindEventtoFacetedGlass (Variables|Default|GetAsWBP_MaterialParameter) (delegate Custom|SetMatFacetedGlass))
  (EventDispatchers|BindEventtoTile (Variables|Default|GetAsWBP_MaterialParameter) (delegate Custom|SetMatCeramicTiles))
  (EventDispatchers|BindEventtoGypsum (Variables|Default|GetAsWBP_MaterialParameter) (delegate Custom|SetMatGypsum))
  (EventDispatchers|BindEventtoDefault (Variables|Default|GetAsWBP_MaterialParameter) (delegate Custom|SetMatDefault))
  (EventDispatchers|BindEventtoDarkGrayFabric (Variables|Default|GetAsWBP_MaterialParameter) (delegate Custom|SetMatDarkGreyFabric))
  (EventDispatchers|BindEventtoPatternedFabric (Variables|Default|GetAsWBP_MaterialParameter) (delegate Custom|SetMatPatternedFabric))
  (EventDispatchers|BindEventtoWhiteCloth (Variables|Default|GetAsWBP_MaterialParameter) (delegate Custom|SetMatWhiteCloth))
  (EventDispatchers|BindEventtoBrownLeather (Variables|Default|GetAsWBP_MaterialParameter) (delegate Custom|SetMatBrownLeather))
  (EventDispatchers|BindEventtoDarkBrownLeather (Variables|Default|GetAsWBP_MaterialParameter) (delegate Custom|SetMatDarkBrownLeather))
  (EventDispatchers|BindEventtoFabricLeather (Variables|Default|GetAsWBP_MaterialParameter) (delegate Custom|SetMatFabricLeather))
  (EventDispatchers|BindEventtoViaLatteaGranite (Variables|Default|GetAsWBP_MaterialParameter) (delegate Custom|SetMatViaLatteaGranite))
  (EventDispatchers|BindEventtoTranslucent (Variables|Default|GetAsWBP_MaterialParameter) (delegate Custom|SetMatTranslucent))
  (EventDispatchers|BindEventtoGlass (Variables|Default|GetAsWBP_MaterialParameter) (delegate Custom|SetMatGlass))
  (EventDispatchers|BindEventtoMetallic (Variables|Default|GetAsWBP_MaterialParameter) (delegate Custom|SetMatMetallic)))

(event Custom|SetMatWood
  ;[1 1 1] Init Dynamic Material Instance
  ;;[1 1 1] Init Bind
  (bind _returnvalue (Rendering|Material|CreateDynamicMaterialInstance "/Game/Material/MI_WoodenFloor.MI_WoodenFloor" "None" "None" :!class /Script/Engine.KismetMaterialLibrary))
  (CallFunction|SetSelectDynamicMaterialInstance _returnvalue (Utilities|Struct|MakeStruct_EnableParameter true false false false false false false false)))

(event Custom|SetMatDefault
  ;[1 1 1] Init Dynamic Material Instance
  ;;[1 1 1] Init Bind
  (bind _returnvalue (Rendering|Material|CreateDynamicMaterialInstance "/Game/Material/MI_Default.MI_Default" "None" "None" :!class /Script/Engine.KismetMaterialLibrary))
  (CallFunction|SetSelectDynamicMaterialInstance _returnvalue (Utilities|Struct|MakeStruct_EnableParameter false true true true true false false true)))

(event Custom|InitMeshSelectButton
  ;[1 1 1] Init Meshes
  ;;[1 1 1] Set Mesh Select Button Enabled
  (for _array_element (Actor|GetComponentsByClass (Variables|Default|GetAsBP_Mesh) "/Script/Engine.StaticMeshComponent")
    (Utilities|IsValid (Variables|/Script/Engine.StaticMeshComponent|GetStaticMesh _array_element)
      (:Is%20Valid
        (Math|Integer|IncrementInt (Variables|Default|GetArray%20Index)))))
  (switch int (Variables|Default|GetArray%20Index)
    (:1
      (Widget|SetIsEnabled (Variables|/Game/Blueprint/Widget/WBP_MeshSelect.WBP_MeshSelect_C|GetMesh06Button (Variables|Default|GetAsWBP%20Mesh%20Select)) false))
    (:2
      (Widget|SetIsEnabled (Variables|/Game/Blueprint/Widget/WBP_MeshSelect.WBP_MeshSelect_C|GetMesh06Button (Variables|Default|GetAsWBP%20Mesh%20Select)) false))
    (:3
      (Widget|SetIsEnabled (Variables|/Game/Blueprint/Widget/WBP_MeshSelect.WBP_MeshSelect_C|GetMesh06Button (Variables|Default|GetAsWBP%20Mesh%20Select)) false))
    (:4
      (Widget|SetIsEnabled (Variables|/Game/Blueprint/Widget/WBP_MeshSelect.WBP_MeshSelect_C|GetMesh06Button (Variables|Default|GetAsWBP%20Mesh%20Select)) false))
    (:5
      (Widget|SetIsEnabled (Variables|/Game/Blueprint/Widget/WBP_MeshSelect.WBP_MeshSelect_C|GetMesh06Button (Variables|Default|GetAsWBP%20Mesh%20Select)) false))
    (:6
      _))
  (Utilities|FlowControl|Sequence
    (:then_0
      ;;[1 1 1] Set Select Mesh
      (if (>= (Variables|Default|GetArray%20Index) 1)
        (EventDispatchers|BindEventtoMesh01 (Variables|Default|GetAsWBP%20Mesh%20Select) (delegate Custom|SetMesh01))
        ;;[1 1 1] Set Default Material
        (bind _returnvalue (Rendering|Material|CreateDynamicMaterialInstance "/Game/Material/MI_Default.MI_Default" "None" "None" :!class /Script/Engine.KismetMaterialLibrary))
        (bind _output_get (Variables|Default|SetMash01SelectMaterial _returnvalue))
        (Rendering|Material|SetMaterial (Variables|/Game/Blueprint/Actor/BP_Mesh.BP_Mesh_C|GetStaticMesh01 (Variables|Default|GetAsBP_Mesh)) 0 _output_get)))
    (:then_1
      (if (>= (Variables|Default|GetArray%20Index) 2)
        (EventDispatchers|BindEventtoMesh02 (Variables|Default|GetAsWBP%20Mesh%20Select) (delegate Custom|SetMesh02))
        (bind _returnvalue_2 (Rendering|Material|CreateDynamicMaterialInstance "/Game/Material/MI_Default.MI_Default" "None" "None" :!class /Script/Engine.KismetMaterialLibrary))
        (bind _output_get_2 (Variables|Default|SetMesh02SelectMaterial _returnvalue_2))
        (Rendering|Material|SetMaterial (Variables|/Game/Blueprint/Actor/BP_Mesh.BP_Mesh_C|GetStaticMesh02 (Variables|Default|GetAsBP_Mesh)) 0 _output_get_2)))
    (:then_2
      (if (>= (Variables|Default|GetArray%20Index) 3)
        (EventDispatchers|BindEventtoMesh03 (Variables|Default|GetAsWBP%20Mesh%20Select) (delegate Custom|SetMesh03))
        (bind _returnvalue_3 (Rendering|Material|CreateDynamicMaterialInstance "/Game/Material/MI_Default.MI_Default" "None" "None" :!class /Script/Engine.KismetMaterialLibrary))
        (bind _output_get_3 (Variables|Default|SetMesh03SelectMaterial _returnvalue_3))
        (Rendering|Material|SetMaterial (Variables|/Game/Blueprint/Actor/BP_Mesh.BP_Mesh_C|GetStaticMesh03 (Variables|Default|GetAsBP_Mesh)) 0 _output_get_3)))
    (:then_3
      (if (>= (Variables|Default|GetArray%20Index) 4)
        (EventDispatchers|BindEventtoMesh04 (Variables|Default|GetAsWBP%20Mesh%20Select) (delegate Custom|SetMesh04))
        (bind _returnvalue_4 (Rendering|Material|CreateDynamicMaterialInstance "/Game/Material/MI_Default.MI_Default" "None" "None" :!class /Script/Engine.KismetMaterialLibrary))
        (bind _output_get_4 (Variables|Default|SetMesh04SelectMaterial _returnvalue_4))
        (Rendering|Material|SetMaterial (Variables|/Game/Blueprint/Actor/BP_Mesh.BP_Mesh_C|GetStaticMesh04 (Variables|Default|GetAsBP_Mesh)) 0 _output_get_4)))
    (:then_4
      (if (>= (Variables|Default|GetArray%20Index) 5)
        (EventDispatchers|BindEventtoMesh05 (Variables|Default|GetAsWBP%20Mesh%20Select) (delegate Custom|SetMesh05))
        (bind _returnvalue_5 (Rendering|Material|CreateDynamicMaterialInstance "/Game/Material/MI_Default.MI_Default" "None" "None" :!class /Script/Engine.KismetMaterialLibrary))
        (bind _output_get_5 (Variables|Default|SetMesh05SelectMaterial _returnvalue_5))
        (Rendering|Material|SetMaterial (Variables|/Game/Blueprint/Actor/BP_Mesh.BP_Mesh_C|GetStaticMesh05 (Variables|Default|GetAsBP_Mesh)) 0 _output_get_5)))
    (:then_5
      (if (>= (Variables|Default|GetArray%20Index) 6)
        (EventDispatchers|BindEventtoMesh06 (Variables|Default|GetAsWBP%20Mesh%20Select) (delegate Custom|SetMesh06))
        (bind _returnvalue_6 (Rendering|Material|CreateDynamicMaterialInstance "/Game/Material/MI_Default.MI_Default" "None" "None" :!class /Script/Engine.KismetMaterialLibrary))
        (bind _output_get_6 (Variables|Default|SetMesh06SelectMaterial _returnvalue_6))
        (Rendering|Material|SetMaterial (Variables|/Game/Blueprint/Actor/BP_Mesh.BP_Mesh_C|GetStaticMesh06 (Variables|Default|GetAsBP_Mesh)) 0 _output_get_6)))))

(event Custom|SetParameterSelectMesh
  (params (SelectDynamicMaterialInstance :type Material%20Instance%20Dynamic%20Object%20Reference))
  (bind _aswbp_materialparameter (Variables|Default|GetAsWBP_MaterialParameter))
  ;[1 1 1] SetParameters
  (Utilities|FlowControl|Sequence
    (:then_0
      ;;[1 1 1] BaseColor
      (bind _value (Default|FNCGetValueBaseColorR _aswbp_materialparameter))
      (bind _value_2 (Default|FNCGetValueBaseColorG _aswbp_materialparameter))
      (bind _value_3 (Default|FNCGetValueBaseColorB _aswbp_materialparameter))
      (Rendering|Material|SetVectorParameterValue SelectDynamicMaterialInstance "BaseColor" (Utilities|Struct|MakeLinearColor _value _value_2 _value_3 1.0) :!class /Script/Engine.MaterialInstanceDynamic))
    (:then_1
      ;;[1 1 1] Metallic
      (bind _value_4 (Default|FNCGetValueMetallic (Variables|Default|GetAsWBP_MaterialParameter)))
      (Rendering|Material|SetScalarParameterValue SelectDynamicMaterialInstance "Metallic" _value_4 :!class /Script/Engine.MaterialInstanceDynamic)
      ;;[1 1 1] Set Emissive
      (bind _value_5 (Default|FNCGetValueEmissive (Variables|Default|GetAsWBP_MaterialParameter)))
      (Rendering|Material|SetScalarParameterValue SelectDynamicMaterialInstance "Emissive" _value_5 :!class /Script/Engine.MaterialInstanceDynamic)
      ;;[1 1 1] Set Roughness
      (bind _value_6 (Default|FNCGetValueRoughness (Variables|Default|GetAsWBP_MaterialParameter)))
      (Rendering|Material|SetScalarParameterValue SelectDynamicMaterialInstance "Roughness" _value_6 :!class /Script/Engine.MaterialInstanceDynamic)
      ;;[1 1 1] Set Refraction
      (bind _value_7 (Default|FNCGetValueRefraction (Variables|Default|GetAsWBP_MaterialParameter)))
      (Rendering|Material|SetScalarParameterValue SelectDynamicMaterialInstance "Refraction" _value_7 :!class /Script/Engine.MaterialInstanceDynamic)
      ;;[1 1 1] Set Opacity
      (bind _value_8 (Default|FNCGetValueOpacity (Variables|Default|GetAsWBP_MaterialParameter)))
      (Rendering|Material|SetScalarParameterValue SelectDynamicMaterialInstance "Opacity" _value_8 :!class /Script/Engine.MaterialInstanceDynamic)
      ;;[1 1 1] Set Specular
      (bind _value_9 (Default|FNCGetValueSpecular (Variables|Default|GetAsWBP_MaterialParameter)))
      (Rendering|Material|SetScalarParameterValue SelectDynamicMaterialInstance "Specular" _value_9 :!class /Script/Engine.MaterialInstanceDynamic))
    (:then_2
      ;;[1 1 1] Set TexCoord
      (bind _value_10 (Default|FNCGetValueTextureTilling (Variables|Default|GetAsWBP_MaterialParameter)))
      (bind _returnvalue (Rendering|Material|GetVectorParameterValue SelectDynamicMaterialInstance "Tiling/Offset" :!class /Script/Engine.MaterialInstanceDynamic))
      (Rendering|Material|SetVectorParameterValue SelectDynamicMaterialInstance "Tiling/Offset" (Utilities|Struct|MakeLinearColor _value_10 _value_10 (.b _returnvalue) (.a _returnvalue)) :!class /Script/Engine.MaterialInstanceDynamic)
      (Rendering|Material|SetScalarParameterValue SelectDynamicMaterialInstance "TexCoord" _value_10 :!class /Script/Engine.MaterialInstanceDynamic)
      (CallFunction|SetStruct _value _value_2 _value_3 _value_5 _value_4 _value_6 _value_10 _value_8 _value_7 _value_9))))

(event Custom|SetMatFacetedGlass
  ;[1 1 1] Init Dynamic Material Instance
  ;;[1 1 1] Init Bind
  (bind _returnvalue (Rendering|Material|CreateDynamicMaterialInstance "/Game/Material/MI_FacetedGlass.MI_FacetedGlass" "None" "None" :!class /Script/Engine.KismetMaterialLibrary))
  (CallFunction|SetSelectDynamicMaterialInstance _returnvalue (Utilities|Struct|MakeStruct_EnableParameter true true false false false false false false)))

(event Custom|SetSliderValue
  (params (SerectStruct :type Struct%20Material%20Parameter%20Structure))
  (bind _aswbp_materialparameter (Variables|Default|GetAsWBP_MaterialParameter))
  ;[1 1 1] Init Meshes
  ;;[1 1 1] Set Parameter Slider Value
  (Class|Slider|SetValue (Variables|/Game/Blueprint/Widget/WBP_MaterialParameter.WBP_MaterialParameter_C|GetSlider_BaseColorR _aswbp_materialparameter) (.basecolorr SerectStruct))
  (Class|Slider|SetValue (Variables|/Game/Blueprint/Widget/WBP_MaterialParameter.WBP_MaterialParameter_C|GetSlider_Roughness _aswbp_materialparameter) (.roughness SerectStruct))
  (Class|Slider|SetValue (Variables|/Game/Blueprint/Widget/WBP_MaterialParameter.WBP_MaterialParameter_C|GetSlider_BaseColorG _aswbp_materialparameter) (.basecolorg SerectStruct))
  (Class|Slider|SetValue (Variables|/Game/Blueprint/Widget/WBP_MaterialParameter.WBP_MaterialParameter_C|GetSlider_TextureTilling _aswbp_materialparameter) (.texturetiling SerectStruct))
  (Class|Slider|SetValue (Variables|/Game/Blueprint/Widget/WBP_MaterialParameter.WBP_MaterialParameter_C|GetSlider_BaseColorB _aswbp_materialparameter) (.basecolorb SerectStruct))
  (Class|Slider|SetValue (Variables|/Game/Blueprint/Widget/WBP_MaterialParameter.WBP_MaterialParameter_C|GetSlider_Opacity _aswbp_materialparameter) (.opacity SerectStruct))
  (Class|Slider|SetValue (Variables|/Game/Blueprint/Widget/WBP_MaterialParameter.WBP_MaterialParameter_C|GetSlider_Emissive _aswbp_materialparameter) (.emissive SerectStruct))
  (Class|Slider|SetValue (Variables|/Game/Blueprint/Widget/WBP_MaterialParameter.WBP_MaterialParameter_C|GetSlider_Refraction _aswbp_materialparameter) (.refraction SerectStruct))
  (Class|Slider|SetValue (Variables|/Game/Blueprint/Widget/WBP_MaterialParameter.WBP_MaterialParameter_C|GetSlider_Metallic _aswbp_materialparameter) (.metallic SerectStruct))
  (Class|Slider|SetValue (Variables|/Game/Blueprint/Widget/WBP_MaterialParameter.WBP_MaterialParameter_C|GetSlider_Specular _aswbp_materialparameter) (.specular SerectStruct)))

(event Custom|InitStruct
  (bind _aswbp_materialparameter (Variables|Default|GetAsWBP_MaterialParameter))
  ;[1 1 1] InitStruct
  (bind _value (Default|FNCGetValueBaseColorR _aswbp_materialparameter))
  (bind _value_2 (Default|FNCGetValueBaseColorB _aswbp_materialparameter))
  (bind _value_3 (Default|FNCGetValueBaseColorG _aswbp_materialparameter))
  (bind _value_4 (Default|FNCGetValueEmissive _aswbp_materialparameter))
  (bind _value_5 (Default|FNCGetValueMetallic _aswbp_materialparameter))
  (bind _value_6 (Default|FNCGetValueRoughness _aswbp_materialparameter))
  (bind _value_7 (Default|FNCGetValueTextureTilling _aswbp_materialparameter))
  (bind _value_8 (Default|FNCGetValueOpacity _aswbp_materialparameter))
  (bind _value_9 (Default|FNCGetValueRefraction _aswbp_materialparameter))
  (bind _value_10 (Default|FNCGetValueSpecular _aswbp_materialparameter))
  (bind _output_get (Variables|Default|SetStructParameterValueMesh01 (Utilities|Struct|MakeStruct_MaterialParameter _value _value_2 _value_3 _value_4 _value_5 _value_6 _value_7 _value_8 _value_9 _value_10)))
  (bind _output_get_2 (Variables|Default|SetStructParameterValueMesh02 _output_get))
  (bind _output_get_3 (Variables|Default|SetStructParameterValueMesh03 _output_get_2))
  (bind _output_get_4 (Variables|Default|SetStructParameterValueMesh04 _output_get_3))
  (bind _output_get_5 (Variables|Default|SetStructParameterValueMesh05 _output_get_4))
  (Variables|Default|SetStructParameterValueMesh06 _output_get_5))

(event Custom|SetMatCeramicTiles
  ;[1 1 1] Init Dynamic Material Instance
  ;;[1 1 1] Init Bind
  (bind _returnvalue (Rendering|Material|CreateDynamicMaterialInstance "/Game/Material/MI_Patterened_Ceramic_Tiles_uk0ocizfw_2K.MI_Patterened_Ceramic_Tiles_uk0ocizfw_2K" "None" "None" :!class /Script/Engine.KismetMaterialLibrary))
  (CallFunction|SetSelectDynamicMaterialInstance _returnvalue (Utilities|Struct|MakeStruct_EnableParameter true false false false false false false false)))

(event EventBeginPlay
  (Utilities|FlowControl|Sequence
    (:then_0
      ;[1 1 1] InitWidget
      (bind _returnvalue (Actor|GetActorOfClass "/Game/Blueprint/Manager/BPM_Widget.BPM_Widget_C"))
      (Variables|Default|SetAsWBP_MaterialParameter (Variables|/Game/Blueprint/Widget/WBP_Widgets.WBP_Widgets_C|GetWBP_MaterialParameter (Variables|/Game/Blueprint/Manager/BPM_Widget.BPM_Widget_C|GetAsWBP_Widget _returnvalue)))
      (Variables|Default|SetAsWBP%20Mesh%20Select (Variables|/Game/Blueprint/Widget/WBP_Widgets.WBP_Widgets_C|GetWBP_MeshSelect (Variables|/Game/Blueprint/Manager/BPM_Widget.BPM_Widget_C|GetAsWBP_Widget _returnvalue))))
    (:then_1
      ;[1 1 1] InitTarget
      (bind _returnvalue_2 (Actor|GetActorOfClass "/Game/Blueprint/Actor/BP_Mesh.BP_Mesh_C"))
      (Variables|Default|SetAsBP_Mesh _returnvalue_2))
    (:then_2
      (CallFunction|InitStruct)
      (CallFunction|InitBind)
      (CallFunction|InitMeshSelectButton))
    (:then_3
      ;[1 1 1] InitDefaultMaterial
      (CallFunction|SetMesh01))))

(event EventTick
  (params (DeltaSeconds :type Float%20%28single-precision%29))
  (if (Variables|Default|GetShowMaterialParameterWindow)
    (switch int (Variables|Default|GetSelectMeshNum)
      (:1
        (CallFunction|SetParameterSelectMesh (Variables|Default|GetMash01SelectMaterial)))
      (:2
        (CallFunction|SetParameterSelectMesh (Variables|Default|GetMesh02SelectMaterial)))
      (:3
        (CallFunction|SetParameterSelectMesh (Variables|Default|GetMesh03SelectMaterial)))
      (:4
        (CallFunction|SetParameterSelectMesh (Variables|Default|GetMesh04SelectMaterial)))
      (:5
        (CallFunction|SetParameterSelectMesh (Variables|Default|GetMesh05SelectMaterial)))
      (:6
        (CallFunction|SetParameterSelectMesh (Variables|Default|GetMesh06SelectMaterial))))))

(fn ConstructionScript)