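; Manager Blueprint for the right-side menu, which edits mesh materials and cine camera settings at runtime.
; BeginPlay creates WBP_RightMenu, finds BP_Mesh and the pawn, and binds mesh, material-preset and camera buttons.
; Presets create dynamic material instances; while the parameter window shows, Tick polls sliders into material and camera, syncing exposure back when automatic.
; Only meshes 1 and 2 store materials and slider values; slots 3–6 just change selection.
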(event Custom|SetAutoExposureOn
  ;[1 1 1] InitCamera
  (Variables|Default|SetAutoExposure true)
  (Variables|/Script/Engine.CameraComponent|SetPostProcessSettings (Variables|/Game/Blueprint/BP_MyPawn.BP_MyPawn_C|GetCineCamera (Variables|Default|GetAs%20BP%20My%20Pawn)) (Utilities|Struct|MakePostProcessSettings "AEM_Histogram")))

(event Custom|SetAutoExposureOff
  ;[1 1 1] InitCamera
  (Variables|Default|SetAutoExposure false)
  (Variables|/Script/Engine.CameraComponent|SetPostProcessSettings (Variables|/Game/Blueprint/BP_MyPawn.BP_MyPawn_C|GetCineCamera (Variables|Default|GetAs%20BP%20My%20Pawn)) (Utilities|Struct|MakePostProcessSettings "AEM_Manual")))

(event Custom|SetMatDarkGreyFabric
  ;[1 1 1] InitDynamicMaterialInstances
  (bind _returnvalue (Rendering|Material|CreateDynamicMaterialInstance "/Game/Material/MI_Dark_Grey_Fabric_sbkla2p0_2K.MI_Dark_Grey_Fabric_sbkla2p0_2K" "None" "None" :!class /Script/Engine.KismetMaterialLibrary))
  (CallFunction|SetSelectDynamicMaterialInstance _returnvalue))

(event Custom|SetMatPatternedFabric
  ;[1 1 1] InitDynamicMaterialInstances
  (bind _returnvalue (Rendering|Material|CreateDynamicMaterialInstance "/Game/Material/MI_Patterned_Fabric_pcvg22p0_2K.MI_Patterned_Fabric_pcvg22p0_2K" "None" "None" :!class /Script/Engine.KismetMaterialLibrary))
  (CallFunction|SetSelectDynamicMaterialInstance _returnvalue))

(event Custom|SetMatWhiteCloth
  ;[1 1 1] InitDynamicMaterialInstances
  (bind _returnvalue (Rendering|Material|CreateDynamicMaterialInstance "/Game/Material/MI_White_Cloth_sbklx0p0_2K.MI_White_Cloth_sbklx0p0_2K" "None" "None" :!class /Script/Engine.KismetMaterialLibrary))
  (CallFunction|SetSelectDynamicMaterialInstance _returnvalue))

(event Custom|SetMatBrownLeather
  ;[1 1 1] InitDynamicMaterialInstances
  (bind _returnvalue (Rendering|Material|CreateDynamicMaterialInstance "/Game/Material/MI_Leather_oizuetp0_2K.MI_Leather_oizuetp0_2K" "None" "None" :!class /Script/Engine.KismetMaterialLibrary))
  (CallFunction|SetSelectDynamicMaterialInstance _returnvalue))

(event Custom|SetMatFabricLeather
  ;[1 1 1] InitDynamicMaterialInstances
  (bind _returnvalue (Rendering|Material|CreateDynamicMaterialInstance "/Game/Material/MI_Fabric_Leather_oizqhap0_2K.MI_Fabric_Leather_oizqhap0_2K" "None" "None" :!class /Script/Engine.KismetMaterialLibrary))
  (CallFunction|SetSelectDynamicMaterialInstance _returnvalue))

(event Custom|SetSelectDynamicMaterialInstance
  (params (SelectDynamicMaterialInstance :type Material%20Instance%20Dynamic%20Object%20Reference))
  (bind _selectmesh (Variables|Default|GetSelectMesh))
  ;[1 1 1] InitDynamicMaterialInstances
  (switch int (Variables|Default|GetSelectMeshNum)
    (:1
      (bind _output_get (Variables|Default|SetMash01SelectMaterial SelectDynamicMaterialInstance))
      (Rendering|Material|SetMaterial _selectmesh 0 _output_get))
    (:2
      (bind _output_get_2 (Variables|Default|SetMesh02SelectMaterial SelectDynamicMaterialInstance))
      (Rendering|Material|SetMaterial _selectmesh 0 _output_get_2))))

(event Custom|SetMatGypsum
  ;[1 1 1] InitDynamicMaterialInstances
  (bind _returnvalue (Rendering|Material|CreateDynamicMaterialInstance "/Game/Material/MI_Gypsum_Tiles_uldnbcdn_2K.MI_Gypsum_Tiles_uldnbcdn_2K" "None" "None" :!class /Script/Engine.KismetMaterialLibrary))
  (CallFunction|SetSelectDynamicMaterialInstance _returnvalue))

(event Custom|SetMatViaLatteaGranite
  ;[1 1 1] InitDynamicMaterialInstances
  (bind _returnvalue (Rendering|Material|CreateDynamicMaterialInstance "/Game/Material/MI_Via_Lattea_Granite_weoldhcv_2K.MI_Via_Lattea_Granite_weoldhcv_2K" "None" "None" :!class /Script/Engine.KismetMaterialLibrary))
  (CallFunction|SetSelectDynamicMaterialInstance _returnvalue))

(event Custom|SetMatDarkBrownLeather
  ;[1 1 1] InitDynamicMaterialInstances
  (bind _returnvalue (Rendering|Material|CreateDynamicMaterialInstance "/Game/Material/MI_Leather_sjqecg1c_2K.MI_Leather_sjqecg1c_2K" "None" "None" :!class /Script/Engine.KismetMaterialLibrary))
  (CallFunction|SetSelectDynamicMaterialInstance _returnvalue))

(event Custom|SetMatTranslucent
  ;[1 1 1] InitDynamicMaterialInstances
  (bind _returnvalue (Rendering|Material|CreateDynamicMaterialInstance "/Game/Material/MI_Translucent.MI_Translucent" "None" "None" :!class /Script/Engine.KismetMaterialLibrary))
  (CallFunction|SetSelectDynamicMaterialInstance _returnvalue))

(event Custom|SetMatDefaultWhite
  ;[1 1 1] InitDynamicMaterialInstances
  (bind _returnvalue (Rendering|Material|CreateDynamicMaterialInstance "/Game/Material/M_DefaultWhite.M_DefaultWhite" "None" "None" :!class /Script/Engine.KismetMaterialLibrary))
  (CallFunction|SetSelectDynamicMaterialInstance _returnvalue))

(event Custom|SetMatGlass
  ;[1 1 1] InitDynamicMaterialInstances
  (bind _returnvalue (Rendering|Material|CreateDynamicMaterialInstance "/Game/Material/MI_Glass.MI_Glass" "None" "None" :!class /Script/Engine.KismetMaterialLibrary))
  (CallFunction|SetSelectDynamicMaterialInstance _returnvalue))

(event Custom|SetMesh02
  ;[1 1 1] InitMeshes
  (Variables|Default|SetSelectMesh (Variables|/Game/Blueprint/Actor/BP_Mesh.BP_Mesh_C|GetStaticMesh02 (Variables|Default|GetAsBP_Mesh)))
  (Variables|Default|SetSelectMeshNum 2)
  (CallFunction|SetSliderValue (Variables|Default|GetStructMesh02)))

(event Custom|SetMesh01
  ;[1 1 1] InitMeshes
  (Variables|Default|SetSelectMesh (Variables|/Game/Blueprint/Actor/BP_Mesh.BP_Mesh_C|GetStaticMesh01 (Variables|Default|GetAsBP_Mesh)))
  (Variables|Default|SetSelectMeshNum 1)
  (CallFunction|SetSliderValue (Variables|Default|GetStructMesh01)))

(event Custom|SetMatMetallic
  ;[1 1 1] InitDynamicMaterialInstances
  (bind _returnvalue (Rendering|Material|CreateDynamicMaterialInstance "/Game/Material/MI_Metallic.MI_Metallic" "None" "None" :!class /Script/Engine.KismetMaterialLibrary))
  (CallFunction|SetSelectDynamicMaterialInstance _returnvalue))

(event Custom|SetMesh03
  ;[1 1 1] InitMeshes
  (Variables|Default|SetSelectMesh (Variables|/Game/Blueprint/Actor/BP_Mesh.BP_Mesh_C|GetStaticMesh03 (Variables|Default|GetAsBP_Mesh)))
  (Variables|Default|SetSelectMeshNum 3))

(event Custom|SetMesh04
  ;[1 1 1] InitMeshes
  (Variables|Default|SetSelectMesh (Variables|/Game/Blueprint/Actor/BP_Mesh.BP_Mesh_C|GetStaticMesh04 (Variables|Default|GetAsBP_Mesh)))
  (Variables|Default|SetSelectMeshNum 4))

(event Custom|SetMesh05
  ;[1 1 1] InitMeshes
  (Variables|Default|SetSelectMesh (Variables|/Game/Blueprint/Actor/BP_Mesh.BP_Mesh_C|GetStaticMesh05 (Variables|Default|GetAsBP_Mesh)))
  (Variables|Default|SetSelectMeshNum 5))

(event Custom|SetMesh06
  ;[1 1 1] InitMeshes
  (Variables|Default|SetSelectMesh (Variables|/Game/Blueprint/Actor/BP_Mesh.BP_Mesh_C|GetStaticMesh06 (Variables|Default|GetAsBP_Mesh)))
  (Variables|Default|SetSelectMeshNum 6))

(event Custom|SetStruct
  (params (BaseColorR :type Float%20%28double-precision%29) (BaseColorG :type Float%20%28double-precision%29) (BaseColorB :type Float%20%28double-precision%29) (Emissive :type Float%20%28double-precision%29) (Metallic :type Float%20%28double-precision%29) (Roughness :type Float%20%28double-precision%29) (TextureTiling :type Float%20%28double-precision%29) (Opacity :type Float%20%28double-precision%29) (Refraction :type Float%20%28double-precision%29) (Specular :type Float%20%28double-precision%29))
  ;[1 1 1] SetParameters
  (switch int (Variables|Default|GetSelectMeshNum)
    (:1
      (Variables|Default|SetStructMesh01 (Utilities|Struct|MakeStruct_MaterialParameter BaseColorR BaseColorG BaseColorB Emissive Metallic Roughness TextureTiling Opacity Refraction Specular)))
    (:2
      (Variables|Default|SetStructMesh02 (Utilities|Struct|MakeStruct_MaterialParameter BaseColorR BaseColorG BaseColorB Emissive Metallic Roughness TextureTiling Opacity Refraction Specular)))))

(event Custom|SetMatDefaultBlack
  ;[1 1 1] InitDynamicMaterialInstances
  (bind _returnvalue (Rendering|Material|CreateDynamicMaterialInstance "/Game/Material/M_DefaultBlack.M_DefaultBlack" "None" "None" :!class /Script/Engine.KismetMaterialLibrary))
  (CallFunction|SetSelectDynamicMaterialInstance _returnvalue))

(event Custom|InitCamera
  (bind _aswbp_camerasetting (Variables|Default|GetAsWBP%20CameraSetting))
  ;[1 1 1] InitCamera
  (EventDispatchers|BindEventtoDepthOfFieldon _aswbp_camerasetting (delegate Custom|SetDepthOfFieldOn))
  (EventDispatchers|BindEventtoDepthOfFieldOff _aswbp_camerasetting (delegate Custom|SetDepthOfFieldOff))
  (EventDispatchers|BindEventtoAutoExposureon _aswbp_camerasetting (delegate Custom|SetAutoExposureOn))
  (EventDispatchers|BindEventtoAutoExposureOff _aswbp_camerasetting (delegate Custom|SetAutoExposureOff)))

(event Custom|InitBind
  ;[1 1 1] InitDynamicMaterialInstances
  (EventDispatchers|BindEventtoWhite (Variables|Default|GetAsWBP_MaterialParameter) (delegate Custom|SetMatDefaultWhite))
  (EventDispatchers|BindEventtoBlack (Variables|Default|GetAsWBP_MaterialParameter) (delegate Custom|SetMatDefaultBlack))
  (EventDispatchers|BindEventtoWood (Variables|Default|GetAsWBP_MaterialParameter) (delegate Custom|SetMatWood))
  (EventDispatchers|BindEventtoFacetedGlass (Variables|Default|GetAsWBP_MaterialParameter) (delegate Custom|SetMatFacetedGlass))
  (EventDispatchers|BindEventtoTile (Variables|Default|GetAsWBP_MaterialParameter) (delegate Custom|SetMatCeramicTiles))
  (EventDispatchers|BindEventtoGypsum (Variables|Default|GetAsWBP_MaterialParameter) (delegate Custom|SetMatGypsum))
  (EventDispatchers|BindEventtoDefault (Variables|Default|GetAsWBP_MaterialParameter) (delegate Custom|SetMatDefault))
  (EventDispatchers|BindEventtoDarkGrayFabric (Variables|Default|GetAsWBP_MaterialParameter) (delegate Custom|SetMatDarkGreyFabric))
  (EventDispatchers|BindEventtoPatternedFabric (Variables|Default|GetAsWBP_MaterialParameter) (delegate Custom|SetMatPatternedFabric))
  (EventDispatchers|BindEventtoWhiteCloth (Variables|Default|GetAsWBP_MaterialParameter) (delegate Custom|SetMatWhiteCloth))
  (EventDispatchers|BindEventtoBrownLeather (Variables|Default|GetAsWBP_MaterialParameter) (delegate Custom|SetMatBrownLeather))
  (EventDispatchers|BindEventtoDarkBrownLeather (Variables|Default|GetAsWBP_MaterialParameter) (delegate Custom|SetMatDarkBrownLeather))
  (EventDispatchers|BindEventtoFabricLeather (Variables|Default|GetAsWBP_MaterialParameter) (delegate Custom|SetMatFabricLeather))
  (EventDispatchers|BindEventtoViaLatteaGranite (Variables|Default|GetAsWBP_MaterialParameter) (delegate Custom|SetMatViaLatteaGranite))
  (EventDispatchers|BindEventtoTranslucent (Variables|Default|GetAsWBP_MaterialParameter) (delegate Custom|SetMatTranslucent))
  (EventDispatchers|BindEventtoGlass (Variables|Default|GetAsWBP_MaterialParameter) (delegate Custom|SetMatGlass))
  (EventDispatchers|BindEventtoMetallic (Variables|Default|GetAsWBP_MaterialParameter) (delegate Custom|SetMatMetallic)))

(event Custom|SetMatWood
  ;[1 1 1] InitDynamicMaterialInstances
  (bind _returnvalue (Rendering|Material|CreateDynamicMaterialInstance "/Game/Material/MI_WoodenFloor.MI_WoodenFloor" "None" "None" :!class /Script/Engine.KismetMaterialLibrary))
  (CallFunction|SetSelectDynamicMaterialInstance _returnvalue))

(event Custom|SetMatDefault
  ;[1 1 1] InitDynamicMaterialInstances
  (bind _returnvalue (Rendering|Material|CreateDynamicMaterialInstance "/Game/Material/MI_Default.MI_Default" "None" "None" :!class /Script/Engine.KismetMaterialLibrary))
  (CallFunction|SetSelectDynamicMaterialInstance _returnvalue))

(event Custom|InitMeshSelectButton
  (bind _aswbp_mesh_select (Variables|Default|GetAsWBP%20Mesh%20Select))
  ;[1 1 1] InitMeshes
  (for _array_element (Actor|GetComponentsByClass (Variables|Default|GetAsBP_Mesh) "/Script/Engine.StaticMeshComponent")
    (Utilities|IsValid (Variables|/Script/Engine.StaticMeshComponent|GetStaticMesh _array_element)
      (:Is%20Valid
        (Math|Integer|IncrementInt (Variables|Default|GetArray%20Index)))))
  (switch int (Variables|Default|GetArray%20Index)
    (:0
      _)
    (:1
      (Widget|SetIsEnabled (Variables|/Game/Blueprint/Widget/WBP_MeshSelect.WBP_MeshSelect_C|GetMesh06Button (Variables|Default|GetAsWBP%20Mesh%20Select)) false))
    (:2
      (Widget|SetIsEnabled (Variables|/Game/Blueprint/Widget/WBP_MeshSelect.WBP_MeshSelect_C|GetMesh06Button (Variables|Default|GetAsWBP%20Mesh%20Select)) false))
    (:3
      (Widget|SetIsEnabled (Variables|/Game/Blueprint/Widget/WBP_MeshSelect.WBP_MeshSelect_C|GetMesh06Button (Variables|Default|GetAsWBP%20Mesh%20Select)) false))
    (:4
      (Widget|SetIsEnabled (Variables|/Game/Blueprint/Widget/WBP_MeshSelect.WBP_MeshSelect_C|GetMesh06Button (Variables|Default|GetAsWBP%20Mesh%20Select)) false))
    (:5
      (Widget|SetIsEnabled (Variables|/Game/Blueprint/Widget/WBP_MeshSelect.WBP_MeshSelect_C|GetMesh06Button (Variables|Default|GetAsWBP%20Mesh%20Select)) false)))
  (EventDispatchers|BindEventtoMesh01 _aswbp_mesh_select (delegate Custom|SetMesh01))
  (EventDispatchers|BindEventtoMesh02 _aswbp_mesh_select (delegate Custom|SetMesh02))
  (EventDispatchers|BindEventtoMesh03 _aswbp_mesh_select (delegate Custom|SetMesh03))
  (EventDispatchers|BindEventtoMesh04 _aswbp_mesh_select (delegate Custom|SetMesh04))
  (EventDispatchers|BindEventtoMesh05 _aswbp_mesh_select (delegate Custom|SetMesh05))
  (EventDispatchers|BindEventtoMesh06 _aswbp_mesh_select (delegate Custom|SetMesh06))
  (CallFunction|SetMesh01))

(event Custom|SetParameterSelectMesh
  (params (SelectDynamicMaterialInstance :type Material%20Instance%20Dynamic%20Object%20Reference))
  (bind _aswbp_materialparameter (Variables|Default|GetAsWBP_MaterialParameter))
  ;[1 1 1] SetParameters
  (Utilities|FlowControl|Sequence
    (:then_0
      (bind _value (Default|FNCGetValueBaseColorR _aswbp_materialparameter))
      (bind _value_2 (Default|FNCGetValueBaseColorG _aswbp_materialparameter))
      (bind _value_3 (Default|FNCGetValueBaseColorB _aswbp_materialparameter))
      (Rendering|Material|SetVectorParameterValue SelectDynamicMaterialInstance "BaseColor" (Utilities|Struct|MakeLinearColor _value _value_2 _value_3 1.0) :!class /Script/Engine.MaterialInstanceDynamic))
    (:then_1
      (bind _value_4 (Default|FNCGetValueMetallic (Variables|Default|GetAsWBP_MaterialParameter)))
      (Rendering|Material|SetScalarParameterValue SelectDynamicMaterialInstance "Metallic" _value_4 :!class /Script/Engine.MaterialInstanceDynamic)
      (bind _value_5 (Default|FNCGetValueEmissive (Variables|Default|GetAsWBP_MaterialParameter)))
      (Rendering|Material|SetScalarParameterValue SelectDynamicMaterialInstance "Emissive" _value_5 :!class /Script/Engine.MaterialInstanceDynamic)
      (bind _value_6 (Default|FNCGetValueRoughness (Variables|Default|GetAsWBP_MaterialParameter)))
      (Rendering|Material|SetScalarParameterValue SelectDynamicMaterialInstance "Roughness" _value_6 :!class /Script/Engine.MaterialInstanceDynamic)
      (bind _value_7 (Default|FNCGetValueRefraction (Variables|Default|GetAsWBP_MaterialParameter)))
      (Rendering|Material|SetScalarParameterValue SelectDynamicMaterialInstance "Refraction" _value_7 :!class /Script/Engine.MaterialInstanceDynamic)
      (bind _value_8 (Default|FNCGetValueTextureTilling (Variables|Default|GetAsWBP_MaterialParameter)))
      (Rendering|Material|SetScalarParameterValue SelectDynamicMaterialInstance "TexCoord" _value_8 :!class /Script/Engine.MaterialInstanceDynamic)
      (bind _value_9 (Default|FNCGetValueOpacity (Variables|Default|GetAsWBP_MaterialParameter)))
      (Rendering|Material|SetScalarParameterValue SelectDynamicMaterialInstance "Opacity" _value_9 :!class /Script/Engine.MaterialInstanceDynamic)
      (bind _value_10 (Default|FNCGetValueSpecular (Variables|Default|GetAsWBP_MaterialParameter)))
      (Rendering|Material|SetScalarParameterValue SelectDynamicMaterialInstance "Specular" _value_10 :!class /Script/Engine.MaterialInstanceDynamic))
    (:then_2
      (bind _value_11 (Default|FNCGetValueTextureTilling (Variables|Default|GetAsWBP_MaterialParameter)))
      (bind _returnvalue (Rendering|Material|GetVectorParameterValue SelectDynamicMaterialInstance "Tiling/Offset" :!class /Script/Engine.MaterialInstanceDynamic))
      (Rendering|Material|SetVectorParameterValue SelectDynamicMaterialInstance "Tiling/Offset" (Utilities|Struct|MakeLinearColor _value_11 _value_11 (.b _returnvalue) (.a _returnvalue)) :!class /Script/Engine.MaterialInstanceDynamic)
      (CallFunction|SetStruct _value _value_2 _value_3 _value_5 _value_4 _value_6 _value_11 _value_9 _value_7 _value_10))))

(event Custom|SetMatFacetedGlass
  ;[1 1 1] InitDynamicMaterialInstances
  (bind _returnvalue (Rendering|Material|CreateDynamicMaterialInstance "/Game/Material/MI_FacetedGlass.MI_FacetedGlass" "None" "None" :!class /Script/Engine.KismetMaterialLibrary))
  (CallFunction|SetSelectDynamicMaterialInstance _returnvalue))

(event Custom|SetSliderValue
  (params (NewParam :type Struct%20Material%20Parameter%20Structure))
  (bind _aswbp_materialparameter (Variables|Default|GetAsWBP_MaterialParameter))
  ;[1 1 1] InitMeshes
  (Class|Slider|SetValue (Variables|/Game/Blueprint/Widget/WBP_MaterialParameter.WBP_MaterialParameter_C|GetSlider_BaseColorR _aswbp_materialparameter) (.basecolorr NewParam))
  (Class|Slider|SetValue (Variables|/Game/Blueprint/Widget/WBP_MaterialParameter.WBP_MaterialParameter_C|GetSlider_Roughness _aswbp_materialparameter) (.roughness NewParam))
  (Class|Slider|SetValue (Variables|/Game/Blueprint/Widget/WBP_MaterialParameter.WBP_MaterialParameter_C|GetSlider_BaseColorG _aswbp_materialparameter) (.basecolorg NewParam))
  (Class|Slider|SetValue (Variables|/Game/Blueprint/Widget/WBP_MaterialParameter.WBP_MaterialParameter_C|GetSlider_TextureTilling _aswbp_materialparameter) (.texturetiling NewParam))
  (Class|Slider|SetValue (Variables|/Game/Blueprint/Widget/WBP_MaterialParameter.WBP_MaterialParameter_C|GetSlider_BaseColorB _aswbp_materialparameter) (.basecolorb NewParam))
  (Class|Slider|SetValue (Variables|/Game/Blueprint/Widget/WBP_MaterialParameter.WBP_MaterialParameter_C|GetSlider_Opacity _aswbp_materialparameter) (.opacity NewParam))
  (Class|Slider|SetValue (Variables|/Game/Blueprint/Widget/WBP_MaterialParameter.WBP_MaterialParameter_C|GetSlider_Emissive _aswbp_materialparameter) (.emissive NewParam))
  (Class|Slider|SetValue (Variables|/Game/Blueprint/Widget/WBP_MaterialParameter.WBP_MaterialParameter_C|GetSlider_Refraction _aswbp_materialparameter) (.refraction NewParam))
  (Class|Slider|SetValue (Variables|/Game/Blueprint/Widget/WBP_MaterialParameter.WBP_MaterialParameter_C|GetSlider_Metallic _aswbp_materialparameter) (.metallic NewParam))
  (Class|Slider|SetValue (Variables|/Game/Blueprint/Widget/WBP_MaterialParameter.WBP_MaterialParameter_C|GetSlider_Specular _aswbp_materialparameter) (.specular NewParam)))

(event Custom|InitStruct
  (bind _aswbp_materialparameter (Variables|Default|GetAsWBP_MaterialParameter))
  ;[1 1 1] InitStruct
  (bind _value (Default|FNCGetValueBaseColorR _aswbp_materialparameter))
  (bind _value_2 (Default|FNCGetValueBaseColorB _aswbp_materialparameter))
  (bind _value_3 (Default|FNCGetValueBaseColorG _aswbp_materialparameter))
  (bind _value_4 (Default|FNCGetValueEmissive _aswbp_materialparameter))
  (bind _value_5 (Default|FNCGetValueMetallic _aswbp_materialparameter))
  (bind _value_6 (Default|FNCGetValueRoughness _aswbp_materialparameter))
  (bind _value_7 (Default|FNCGetValueTextureTilling _aswbp_materialparameter))
  (bind _value_8 (Default|FNCGetValueOpacity _aswbp_materialparameter))
  (bind _value_9 (Default|FNCGetValueRefraction _aswbp_materialparameter))
  (bind _value_10 (Default|FNCGetValueSpecular _aswbp_materialparameter))
  (bind _output_get (Variables|Default|SetStructMesh01 (Utilities|Struct|MakeStruct_MaterialParameter _value _value_2 _value_3 _value_4 _value_5 _value_6 _value_7 _value_8 _value_9 _value_10)))
  (Variables|Default|SetStructMesh02 _output_get))

(event Custom|SetMatCeramicTiles
  ;[1 1 1] InitDynamicMaterialInstances
  (bind _returnvalue (Rendering|Material|CreateDynamicMaterialInstance "/Game/Material/MI_Patterened_Ceramic_Tiles_uk0ocizfw_2K.MI_Patterened_Ceramic_Tiles_uk0ocizfw_2K" "None" "None" :!class /Script/Engine.KismetMaterialLibrary))
  (CallFunction|SetSelectDynamicMaterialInstance _returnvalue))

(event Custom|SetDepthOfFieldOn
  ;[1 1 1] InitCamera
  (Variables|/Script/CinematicCamera.CineCameraComponent|SetFocusSettings (Variables|/Game/Blueprint/BP_MyPawn.BP_MyPawn_C|GetCineCamera (Variables|Default|GetAs%20BP%20My%20Pawn)) (Variables|Default|GetFocusSettingTracking)))

(event Custom|SetDepthOfFieldOff
  ;[1 1 1] InitCamera
  (Variables|/Script/CinematicCamera.CineCameraComponent|SetFocusSettings (Variables|/Game/Blueprint/BP_MyPawn.BP_MyPawn_C|GetCineCamera (Variables|Default|GetAs%20BP%20My%20Pawn)) (Variables|Default|GetFocusSettingDisable)))

(event EventBeginPlay
  (Utilities|FlowControl|Sequence
    (:then_0
      ;[1 1 1] InitWidget
      (bind _returnvalue (UserInterface|CreateWidget "/Game/Blueprint/Widget/WBP_RightMenu.WBP_RightMenu_C"))
      (bind _output_get (Variables|Default|SetAsWBP_RightMenu _returnvalue))
      (UserInterface|Viewport|AddtoViewport _output_get 0)
      (Variables|Default|SetAsWBP_MaterialParameter (Variables|/Game/Blueprint/Widget/WBP_RightMenu.WBP_RightMenu_C|GetWBP_MaterialParameter _output_get))
      (Variables|Default|SetAsWBP%20CameraSetting (Variables|/Game/Blueprint/Widget/WBP_RightMenu.WBP_RightMenu_C|GetWBP_CameraSetting _output_get))
      (Variables|Default|SetAsWBP%20Mesh%20Select (Variables|/Game/Blueprint/Widget/WBP_RightMenu.WBP_RightMenu_C|GetWBP_MeshSelect _output_get)))
    (:then_1
      ;[1 1 1] InitTarget
      (bind _returnvalue_2 (Actor|GetActorOfClass "/Game/Blueprint/Actor/BP_Mesh.BP_Mesh_C"))
      (Variables|Default|SetAsBP_Mesh _returnvalue_2)
      (bind _asbp_my_pawn (Utilities|Casting|CastToBP_MyPawn (Game|Player|GetPlayerPawn 0)))
      (Variables|Default|SetAs%20BP%20My%20Pawn _asbp_my_pawn))
    (:then_2
      ;[1 1 1] InitDefaultMaterial
      (bind _returnvalue_3 (Rendering|Material|CreateDynamicMaterialInstance "/Game/Material/MI_Default.MI_Default" "None" "None" :!class /Script/Engine.KismetMaterialLibrary))
      (bind _output_get_2 (Variables|Default|SetMash01SelectMaterial _returnvalue_3))
      (Rendering|Material|SetMaterial (Variables|/Game/Blueprint/Actor/BP_Mesh.BP_Mesh_C|GetStaticMesh01 (Variables|Default|GetAsBP_Mesh)) 0 _output_get_2)
      (bind _returnvalue_4 (Rendering|Material|CreateDynamicMaterialInstance "/Game/Material/MI_Default.MI_Default" "None" "None" :!class /Script/Engine.KismetMaterialLibrary))
      (bind _output_get_3 (Variables|Default|SetMesh02SelectMaterial _returnvalue_4))
      (Rendering|Material|SetMaterial (Variables|/Game/Blueprint/Actor/BP_Mesh.BP_Mesh_C|GetStaticMesh02 (Variables|Default|GetAsBP_Mesh)) 0 _output_get_3))
    (:then_3
      (CallFunction|InitStruct)
      (CallFunction|InitBind)
      (CallFunction|InitMeshSelectButton)
      (CallFunction|InitCamera))))

(event EventTick
  (params (DeltaSeconds :type Float%20%28single-precision%29))
  (if (Variables|Default|GetShowMaterialParameterWindow)
    (Utilities|FlowControl|Sequence
      (:then_0
        (switch int (Variables|Default|GetSelectMeshNum)
          (:1
            (CallFunction|SetParameterSelectMesh (Variables|Default|GetMash01SelectMaterial)))
          (:2
            (CallFunction|SetParameterSelectMesh (Variables|Default|GetMesh02SelectMaterial)))))
      (:then_1
        (Utilities|FlowControl|Sequence
          (:then_0
            ;[1 1 1] CameraSetting
            (bind _value (Default|FNCGetValueCurrentFocusLength (Variables|Default|GetAsWBP%20CameraSetting)))
            (Variables|/Script/CinematicCamera.CineCameraComponent|SetCurrentFocalLength (Variables|/Game/Blueprint/BP_MyPawn.BP_MyPawn_C|GetCineCamera (Variables|Default|GetAs%20BP%20My%20Pawn)) _value)
            (if (Variables|Default|GetAutoExposure)
              (Default|FNCSetValueAutoExposureBias (Variables|Default|GetAsWBP%20CameraSetting) (Utilities|Struct|BreakPostProcessSettings (Variables|/Script/Engine.CameraComponent|GetPostProcessSettings (Variables|/Game/Blueprint/BP_MyPawn.BP_MyPawn_C|GetCineCamera (Variables|Default|GetAs%20BP%20My%20Pawn)))))
              (else
                (bind _value_2 (Default|FNCGetValueAutoExposureBias (Variables|Default|GetAsWBP%20CameraSetting)))
                (Variables|/Script/Engine.CameraComponent|SetPostProcessSettings (Variables|/Game/Blueprint/BP_MyPawn.BP_MyPawn_C|GetCineCamera (Variables|Default|GetAs%20BP%20My%20Pawn)) (Utilities|Struct|MakePostProcessSettings _value_2))))))))))

(fn ConstructionScript)