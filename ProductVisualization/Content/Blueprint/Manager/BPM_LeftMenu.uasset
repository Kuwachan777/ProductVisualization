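; Manager Blueprint for the left menu, which offers screenshot capture and sun controls.
; On BeginPlay it creates WBP_LeftMenu, binds its screenshot and sun-height sub-widget events, finds the level's SunSky and enables its atmosphere sun light.
; Screenshot events run HighResShot console commands at Full HD or 4K, while solar-time events toggle the atmosphere sun light.
; Tick polls the sun-height widget and applies its value as the directional light's pitch.
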(event Custom|FullHDShot
  ;[1 1 1] Init Screen Shot
  (Development|ExecuteConsoleCommand "HighResShot 1920x1080" 0))

(event Custom|4KShot
  ;[1 1 1] Init Screen Shot
  (Development|ExecuteConsoleCommand "HighResShot 3840x2160" 0))

(event Custom|SolarTimeOn
  ;[1 1 1] Init Sun Setting
  (Class|DirectionalLightComponent|SetAtmosphereSunLight (Variables|/SunPosition/SunSky.SunSky_C|GetDirectionalLight (Variables|Default|GetAsSunSky)) true))

(event Custom|SolarTimeOff
  ;[1 1 1] Init Sun Setting
  (Class|DirectionalLightComponent|SetAtmosphereSunLight (Variables|/SunPosition/SunSky.SunSky_C|GetDirectionalLight (Variables|Default|GetAsSunSky)) false))

(event Custom|SunSetting
  (bind _assunsky (Variables|Default|GetAsSunSky))
  (bind _directionallight (Variables|/SunPosition/SunSky.SunSky_C|GetDirectionalLight _assunsky))
  (bind _value (Default|FNCGetValueSunHight (Variables|Default|GetWBP%20Sun%20Hight)))
  (Transformation|SetWorldRotation _directionallight (Math|Rotator|MakeRotator (.roll (Transformation|GetWorldRotation _directionallight)) _value 0.0) false false))

(event Custom|InitWidget
  ;[1 1 1] Create Widget
  (bind _returnvalue (UserInterface|CreateWidget "/Game/Blueprint/Widget/WBP_LeftMenu.WBP_LeftMenu_C"))
  (UserInterface|Viewport|AddtoViewport _returnvalue 0)
  (Variables|Default|SetWBP%20Screen%20Shot (Variables|/Game/Blueprint/Widget/WBP_LeftMenu.WBP_LeftMenu_C|GetWBP_ScreenShot _returnvalue))
  (Variables|Default|SetWBP%20Sun%20Hight (Variables|/Game/Blueprint/Widget/WBP_LeftMenu.WBP_LeftMenu_C|GetWBP_SunHight _returnvalue)))

(event Custom|InitScreenShot
  (bind _wbp_screen_shot (Variables|Default|GetWBP%20Screen%20Shot))
  ;[1 1 1] Init Screen Shot
  (EventDispatchers|BindEventtoFullHDShot _wbp_screen_shot (delegate Custom|FullHDShot))
  (EventDispatchers|BindEventto4KShot _wbp_screen_shot (delegate Custom|4KShot)))

(event Custom|InitSunSetting
  (bind _wbp_sun_hight (Variables|Default|GetWBP%20Sun%20Hight))
  ;[1 1 1] Init Sun Setting
  (Utilities|FlowControl|Sequence
    (:then_0
      (bind _outactors (Actor|GetAllActorsOfClass "/SunPosition/SunSky.SunSky_C"))
      (for _array_element _outactors
        (Variables|Default|SetAsSunSky _array_element)))
    (:then_1
      (EventDispatchers|BindEventtoSolarTimeon _wbp_sun_hight (delegate Custom|SolarTimeOn))
      (EventDispatchers|BindEventtoSolarTimeOff _wbp_sun_hight (delegate Custom|SolarTimeOff)))))

(event EventBeginPlay
  (Utilities|FlowControl|Sequence
    (:then_0
      (CallFunction|InitWidget)
      (CallFunction|InitScreenShot)
      (CallFunction|InitSunSetting))
    (:then_1
      (CallFunction|SolarTimeon))))

(event Collision|EventActorBeginOverlap
  (params (OtherActor :type Actor%20Object%20Reference)))

(event EventTick
  (params (DeltaSeconds :type Float%20%28single-precision%29))
  (CallFunction|SunSetting))

(fn ConstructionScript)