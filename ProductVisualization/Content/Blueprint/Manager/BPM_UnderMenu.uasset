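; Manager Blueprint that drives the under-menu UI for changing floor and screen appearance in the level.
; On BeginPlay it finds BP_Floor and BP_Screen, resets both to default white, and creates WBP_UnderMenu.
; It binds the menu's floor-texture and screen sub-widget dispatchers to its own events.
; Those events swap materials on the floor and both screen meshes, or show and hide the screen actor.
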(event Custom|SetFloorMatDefaultBlack
  (Rendering|Material|SetMaterial (Variables|/Game/Blueprint/Actor/BP_Floor.BP_Floor_C|GetFloor (Variables|Default|GetAsBP_Floor)) 0 "/Game/Material/M_DefaultBlack.M_DefaultBlack"))

(event Custom|SetFloorMatDefaultWhite
  (Rendering|Material|SetMaterial (Variables|/Game/Blueprint/Actor/BP_Floor.BP_Floor_C|GetFloor (Variables|Default|GetAsBP_Floor)) 0 "/Game/Material/M_DefaultWhite.M_DefaultWhite"))

(event Custom|SetScreenMatMetallicBlack
  (Rendering|Material|SetMaterial (Variables|/Game/Blueprint/Actor/BP_Screen.BP_Screen_C|GetScreen (Variables|Default|GetAsBP_Screen)) 0 "/Game/Material/M_MetallicBlack.M_MetallicBlack"))

(event Custom|SetScreenMatWoodFloor
  (Rendering|Material|SetMaterial (Variables|/Game/Blueprint/Actor/BP_Screen.BP_Screen_C|GetScreen (Variables|Default|GetAsBP_Screen)) 0 "/Game/Material/MI_WoodenFloor.MI_WoodenFloor"))

(event Custom|SetFloorMatMetallicBlack
  (Rendering|Material|SetMaterial (Variables|/Game/Blueprint/Actor/BP_Floor.BP_Floor_C|GetFloor (Variables|Default|GetAsBP_Floor)) 0 "/Game/Material/M_MetallicBlack.M_MetallicBlack"))

(event Custom|SetFloorMatGypsum
  (Rendering|Material|SetMaterial (Variables|/Game/Blueprint/Actor/BP_Floor.BP_Floor_C|GetFloor (Variables|Default|GetAsBP_Floor)) 0 "/Game/Material/MI_Gypsum_Tiles_uldnbcdn_2K.MI_Gypsum_Tiles_uldnbcdn_2K"))

(event Custom|SetFloorMatViaLatteaGranite
  (Rendering|Material|SetMaterial (Variables|/Game/Blueprint/Actor/BP_Floor.BP_Floor_C|GetFloor (Variables|Default|GetAsBP_Floor)) 0 "/Game/Material/MI_Via_Lattea_Granite_weoldhcv_2K.MI_Via_Lattea_Granite_weoldhcv_2K"))

(event Custom|SetFloorMatNone
  (Rendering|Material|SetMaterial (Variables|/Game/Blueprint/Actor/BP_Floor.BP_Floor_C|GetFloor (Variables|Default|GetAsBP_Floor)) 0 "/Game/Material/M_Clear.M_Clear"))

(event Custom|SetFloorMatForestFloor
  (Rendering|Material|SetMaterial (Variables|/Game/Blueprint/Actor/BP_Floor.BP_Floor_C|GetFloor (Variables|Default|GetAsBP_Floor)) 0 "/Game/Material/MI_Forest_Floor_vmhkbcug_2K.MI_Forest_Floor_vmhkbcug_2K"))

(event Custom|SetFloorMatWoodenPlank
  (Rendering|Material|SetMaterial (Variables|/Game/Blueprint/Actor/BP_Floor.BP_Floor_C|GetFloor (Variables|Default|GetAsBP_Floor)) 0 "/Game/Material/MI_Wooden_Planks_vgwnadk_2K.MI_Wooden_Planks_vgwnadk_2K"))

(event Custom|SetScreenMatStoneWall
  (Rendering|Material|SetMaterial (Variables|/Game/Blueprint/Actor/BP_Screen.BP_Screen_C|GetScreen (Variables|Default|GetAsBP_Screen)) 0 "/Game/Material/MI_Stone_Wall_vlswfjc_2K.MI_Stone_Wall_vlswfjc_2K"))

(event Custom|SetScreenMatGypsum
  (Rendering|Material|SetMaterial (Variables|/Game/Blueprint/Actor/BP_Screen.BP_Screen_C|GetScreen (Variables|Default|GetAsBP_Screen)) 0 "/Game/Material/MI_Gypsum_Tiles_uldnbcdn_2K.MI_Gypsum_Tiles_uldnbcdn_2K"))

(event Custom|SetFloorMatWoodenFloor
  (Rendering|Material|SetMaterial (Variables|/Game/Blueprint/Actor/BP_Floor.BP_Floor_C|GetFloor (Variables|Default|GetAsBP_Floor)) 0 "/Game/Material/MI_WoodenFloor.MI_WoodenFloor"))

(event Custom|SetScreenMatWoodenPlankWall
  (Rendering|Material|SetMaterial (Variables|/Game/Blueprint/Actor/BP_Screen.BP_Screen_C|GetScreen (Variables|Default|GetAsBP_Screen)) 0 "/Game/Material/MI_Wooden_Planks_Wall_vmchejun_2K.MI_Wooden_Planks_Wall_vmchejun_2K"))

(event Custom|SetScreenMatDarkGreyFabric
  (Rendering|Material|SetMaterial (Variables|/Game/Blueprint/Actor/BP_Screen.BP_Screen_C|GetScreen (Variables|Default|GetAsBP_Screen)) 0 "/Game/Material/MI_Dark_Grey_Fabric_sbkla2p0_2K.MI_Dark_Grey_Fabric_sbkla2p0_2K"))

(event Custom|SetScreenMatViaLatteaGranite
  (Rendering|Material|SetMaterial (Variables|/Game/Blueprint/Actor/BP_Screen.BP_Screen_C|GetScreen (Variables|Default|GetAsBP_Screen)) 0 "/Game/Material/MI_Via_Lattea_Granite_weoldhcv_2K.MI_Via_Lattea_Granite_weoldhcv_2K"))

(event Custom|SetFloorMatCeramicTiles
  (Rendering|Material|SetMaterial (Variables|/Game/Blueprint/Actor/BP_Floor.BP_Floor_C|GetFloor (Variables|Default|GetAsBP_Floor)) 0 "/Game/Material/MI_Patterened_Ceramic_Tiles_uk0ocizfw_2K.MI_Patterened_Ceramic_Tiles_uk0ocizfw_2K"))

(event Custom|SetFloorMatDarkGreyFabric
  (Rendering|Material|SetMaterial (Variables|/Game/Blueprint/Actor/BP_Floor.BP_Floor_C|GetFloor (Variables|Default|GetAsBP_Floor)) 0 "/Game/Material/MI_Dark_Grey_Fabric_sbkla2p0_2K.MI_Dark_Grey_Fabric_sbkla2p0_2K"))

(event Custom|HideScreen
  (Rendering|SetActorHiddenInGame (Variables|Default|GetAsBP_Screen) true))

(event Custom|ShowScreen
  (Rendering|SetActorHiddenInGame (Variables|Default|GetAsBP_Screen) false))

(event Custom|SetScreenMatDefaultWhite
  (Rendering|Material|SetMaterial (Variables|/Game/Blueprint/Actor/BP_Screen.BP_Screen_C|GetScreen (Variables|Default|GetAsBP_Screen)) 0 "/Game/Material/M_DefaultWhite.M_DefaultWhite"))

(event Custom|SetScreenMatDefaultBlack
  (Rendering|Material|SetMaterial (Variables|/Game/Blueprint/Actor/BP_Screen.BP_Screen_C|GetScreen (Variables|Default|GetAsBP_Screen)) 0 "/Game/Material/M_DefaultBlack.M_DefaultBlack"))

(event Custom|SetScreenMatCeramicTiles
  (Rendering|Material|SetMaterial (Variables|/Game/Blueprint/Actor/BP_Screen.BP_Screen_C|GetScreen (Variables|Default|GetAsBP_Screen)) 0 "/Game/Material/MI_Patterened_Ceramic_Tiles_uk0ocizfw_2K.MI_Patterened_Ceramic_Tiles_uk0ocizfw_2K"))

(event EventBeginPlay
  (Utilities|FlowControl|Sequence
    (:then_0
      (bind _returnvalue (Actor|GetActorOfClass "/Game/Blueprint/Actor/BP_Floor.BP_Floor_C"))
      (bind _output_get (Variables|Default|SetAsBP_Floor _returnvalue))
      (Rendering|Material|SetMaterial (Variables|/Game/Blueprint/Actor/BP_Floor.BP_Floor_C|GetFloor _output_get) 0 "/Game/Material/M_DefaultWhite.M_DefaultWhite")
      (bind _returnvalue_2 (Actor|GetActorOfClass "/Game/Blueprint/Actor/BP_Screen.BP_Screen_C"))
      (bind _output_get_2 (Variables|Default|SetAsBP_Screen _returnvalue_2))
      (Rendering|Material|SetMaterial (Variables|/Game/Blueprint/Actor/BP_Screen.BP_Screen_C|GetScreen _output_get_2) 0 "/Game/Material/M_DefaultWhite.M_DefaultWhite"))
    (:then_1
      (bind _returnvalue_3 (UserInterface|CreateWidget "/Game/Blueprint/Widget/WBP_UnderMenu.WBP_UnderMenu_C"))
      (bind _output_get_3 (Variables|Default|SetAsWBP_UnderMenu _returnvalue_3))
      (UserInterface|Viewport|AddtoViewport _output_get_3 0)
      (bind _output_get_4 (Variables|Default|SetAsWBP_FloorTexture (Variables|/Game/Blueprint/Widget/WBP_UnderMenu.WBP_UnderMenu_C|GetWBP_FloorTexture _output_get_3)))
      (EventDispatchers|BindEventtoDefaultBlack _output_get_4 (delegate Custom|SetFloorMatDefaultBlack))
      (EventDispatchers|BindEventtoDefaultWhite _output_get_4 (delegate Custom|SetFloorMatDefaultWhite))
      (EventDispatchers|BindEventtoWoodenFloor _output_get_4 (delegate Custom|SetFloorMatWoodenFloor))
      (EventDispatchers|BindEventtoCeramicTiles _output_get_4 (delegate Custom|SetFloorMatCeramicTiles))
      (EventDispatchers|BindEventtoMetallicBlack _output_get_4 (delegate Custom|SetFloorMatMetallicBlack))
      (EventDispatchers|BindEventtoDarkGreyFabric _output_get_4 (delegate Custom|SetFloorMatDarkGreyFabric))
      (EventDispatchers|BindEventtoViaLatteaGranite _output_get_4 (delegate Custom|SetFloorMatViaLatteaGranite))
      (EventDispatchers|BindEventtoNoneMat _output_get_4 (delegate Custom|SetFloorMatNone))
      (EventDispatchers|BindEventtoForestFloor _output_get_4 (delegate Custom|SetFloorMatForestFloor))
      (EventDispatchers|BindEventtoWoodenPlank _output_get_4 (delegate Custom|SetFloorMatWoodenPlank))
      (EventDispatchers|BindEventtoGypsum _output_get_4 (delegate Custom|SetFloorMatGypsum)))
    (:then_2
      (bind _output_get_5 (Variables|Default|SetWBP%20Screen (Variables|/Game/Blueprint/Widget/WBP_UnderMenu.WBP_UnderMenu_C|GetWBP_Screen _output_get_3)))
      (EventDispatchers|BindEventtoHideScreen _output_get_5 (delegate Custom|HideScreen))
      (EventDispatchers|BindEventtoShowScreen _output_get_5 (delegate Custom|ShowScreen))
      (EventDispatchers|BindEventtoDefaultWhite _output_get_5 (delegate Custom|SetScreenMatDefaultWhite))
      (EventDispatchers|BindEventtoDefaultBlack _output_get_5 (delegate Custom|SetScreenMatDefaultBlack))
      (EventDispatchers|BindEventtoCeramicTiles _output_get_5 (delegate Custom|SetScreenMatCeramicTiles))
      (EventDispatchers|BindEventtoMetallicBlack _output_get_5 (delegate Custom|SetScreenMatMetallicBlack))
      (EventDispatchers|BindEventtoWoodenWall _output_get_5 (delegate Custom|SetScreenMatWoodFloor))
      (EventDispatchers|BindEventtoStoneWall _output_get_5 (delegate Custom|SetScreenMatStoneWall))
      (EventDispatchers|BindEventtoWoodenPlankWall _output_get_5 (delegate Custom|SetScreenMatWoodenPlankWall))
      (EventDispatchers|BindEventtoDarkGreyFabric _output_get_5 (delegate Custom|SetScreenMatDarkGreyFabric))
      (EventDispatchers|BindEventtoViaLatteaGranite _output_get_5 (delegate Custom|SetScreenMatViaLatteaGranite))
      (EventDispatchers|BindEventtoGypsum _output_get_5 (delegate Custom|SetScreenMatGypsum)))))

(event Collision|EventActorBeginOverlap
  (params (OtherActor :type Actor%20Object%20Reference)))

(event EventTick
  (params (DeltaSeconds :type Float%20%28single-precision%29)))

(fn ConstructionScript)