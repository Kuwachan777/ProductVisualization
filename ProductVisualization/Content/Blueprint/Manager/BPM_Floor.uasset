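; Floor manager Blueprint that changes the material and visibility of the level's BP_Floor actor from the floor settings UI.
; On BeginPlay it finds the WBPFloorSetting widget through BPM_Widget, caches BP_Floor and applies a default white material.
; It then binds the widget's events to handlers that each set a preset material on the Floor component's first slot or show and hide the actor in game.
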(event Custom|SetFloorMatDefaultBlack
  (Rendering|Material|SetMaterial (Variables|/Game/Blueprint/Actor/BP_Floor.BP_Floor_C|GetFloor (Variables|Default|GetAsBP_Floor)) 0 "/Game/Material/M_DefaultBlack.M_DefaultBlack"))

(event Custom|SetFloorMatDefaultWhite
  (Rendering|Material|SetMaterial (Variables|/Game/Blueprint/Actor/BP_Floor.BP_Floor_C|GetFloor (Variables|Default|GetAsBP_Floor)) 0 "/Game/Material/M_DefaultWhite.M_DefaultWhite"))

(event Custom|SetFloorMatMetallicBlack
  (Rendering|Material|SetMaterial (Variables|/Game/Blueprint/Actor/BP_Floor.BP_Floor_C|GetFloor (Variables|Default|GetAsBP_Floor)) 0 "/Game/Material/M_MetallicBlack.M_MetallicBlack"))

(event Custom|SetFloorMatGypsum
  (Rendering|Material|SetMaterial (Variables|/Game/Blueprint/Actor/BP_Floor.BP_Floor_C|GetFloor (Variables|Default|GetAsBP_Floor)) 0 "/Game/Material/MI_Gypsum_Tiles_uldnbcdn_2K.MI_Gypsum_Tiles_uldnbcdn_2K"))

(event Custom|SetFloorMatViaLatteaGranite
  (Rendering|Material|SetMaterial (Variables|/Game/Blueprint/Actor/BP_Floor.BP_Floor_C|GetFloor (Variables|Default|GetAsBP_Floor)) 0 "/Game/Material/MI_Via_Lattea_Granite_weoldhcv_2K.MI_Via_Lattea_Granite_weoldhcv_2K"))

(event Custom|HiddenFloor
  (Rendering|SetActorHiddenInGame (Variables|Default|GetAsBP_Floor) true))

(event Custom|SetFloorMatForestFloor
  (Rendering|Material|SetMaterial (Variables|/Game/Blueprint/Actor/BP_Floor.BP_Floor_C|GetFloor (Variables|Default|GetAsBP_Floor)) 0 "/Game/Material/MI_Forest_Floor_vmhkbcug_2K.MI_Forest_Floor_vmhkbcug_2K"))

(event Custom|SetFloorMatWoodenPlank
  (Rendering|Material|SetMaterial (Variables|/Game/Blueprint/Actor/BP_Floor.BP_Floor_C|GetFloor (Variables|Default|GetAsBP_Floor)) 0 "/Game/Material/MI_Wooden_Planks_vgwnadk_2K.MI_Wooden_Planks_vgwnadk_2K"))

(event Custom|SetFloorMatWoodenFloor
  (Rendering|Material|SetMaterial (Variables|/Game/Blueprint/Actor/BP_Floor.BP_Floor_C|GetFloor (Variables|Default|GetAsBP_Floor)) 0 "/Game/Material/MI_WoodenFloor.MI_WoodenFloor"))

(event Custom|ShowFloor
  (Rendering|SetActorHiddenInGame (Variables|Default|GetAsBP_Floor) false))

(event Custom|SetFloorMatCeramicTiles
  (Rendering|Material|SetMaterial (Variables|/Game/Blueprint/Actor/BP_Floor.BP_Floor_C|GetFloor (Variables|Default|GetAsBP_Floor)) 0 "/Game/Material/MI_Patterened_Ceramic_Tiles_uk0ocizfw_2K.MI_Patterened_Ceramic_Tiles_uk0ocizfw_2K"))

(event Custom|SetFloorMatDarkGreyFabric
  (Rendering|Material|SetMaterial (Variables|/Game/Blueprint/Actor/BP_Floor.BP_Floor_C|GetFloor (Variables|Default|GetAsBP_Floor)) 0 "/Game/Material/MI_Dark_Grey_Fabric_sbkla2p0_2K.MI_Dark_Grey_Fabric_sbkla2p0_2K"))

(event EventBeginPlay
  (Utilities|FlowControl|Sequence
    (:then_0
      (bind _returnvalue (Actor|GetActorOfClass "/Game/Blueprint/Manager/BPM_Widget.BPM_Widget_C"))
      (Variables|Default|SetAsWBP_FloorSetting (Variables|/Game/Blueprint/Widget/WBP_Widgets.WBP_Widgets_C|GetWBP_FloorSetting (Variables|/Game/Blueprint/Manager/BPM_Widget.BPM_Widget_C|GetAsWBP_Widget _returnvalue))))
    (:then_1
      (bind _returnvalue_2 (Actor|GetActorOfClass "/Game/Blueprint/Actor/BP_Floor.BP_Floor_C"))
      (bind _output_get (Variables|Default|SetAsBP_Floor _returnvalue_2))
      (Rendering|Material|SetMaterial (Variables|/Game/Blueprint/Actor/BP_Floor.BP_Floor_C|GetFloor _output_get) 0 "/Game/Material/M_DefaultWhite.M_DefaultWhite"))
    (:then_2
      (EventDispatchers|BindEventtoDefaultBlack (Variables|Default|GetAsWBP_FloorSetting) (delegate Custom|SetFloorMatDefaultBlack))
      (EventDispatchers|BindEventtoDefaultWhite (Variables|Default|GetAsWBP_FloorSetting) (delegate Custom|SetFloorMatDefaultWhite))
      (EventDispatchers|BindEventtoWoodenFloor (Variables|Default|GetAsWBP_FloorSetting) (delegate Custom|SetFloorMatWoodenFloor))
      (EventDispatchers|BindEventtoCeramicTiles (Variables|Default|GetAsWBP_FloorSetting) (delegate Custom|SetFloorMatCeramicTiles))
      (EventDispatchers|BindEventtoMetallicBlack (Variables|Default|GetAsWBP_FloorSetting) (delegate Custom|SetFloorMatMetallicBlack))
      (EventDispatchers|BindEventtoDarkGreyFabric (Variables|Default|GetAsWBP_FloorSetting) (delegate Custom|SetFloorMatDarkGreyFabric))
      (EventDispatchers|BindEventtoViaLatteaGranite (Variables|Default|GetAsWBP_FloorSetting) (delegate Custom|SetFloorMatViaLatteaGranite))
      (EventDispatchers|BindEventtoForestFloor (Variables|Default|GetAsWBP_FloorSetting) (delegate Custom|SetFloorMatForestFloor))
      (EventDispatchers|BindEventtoWoodenPlank (Variables|Default|GetAsWBP_FloorSetting) (delegate Custom|SetFloorMatWoodenPlank))
      (EventDispatchers|BindEventtoGypsum (Variables|Default|GetAsWBP_FloorSetting) (delegate Custom|SetFloorMatGypsum))
      (EventDispatchers|BindEventtoShowFloor (Variables|Default|GetAsWBP_FloorSetting) (delegate Custom|ShowFloor))
      (EventDispatchers|BindEventtoHiddenFloor (Variables|Default|GetAsWBP_FloorSetting) (delegate Custom|HiddenFloor)))))

(event Collision|EventActorBeginOverlap
  (params (OtherActor :type Actor%20Object%20Reference)))

(event EventTick
  (params (DeltaSeconds :type Float%20%28single-precision%29)))

(fn ConstructionScript)