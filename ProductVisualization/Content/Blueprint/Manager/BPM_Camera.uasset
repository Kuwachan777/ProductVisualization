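; Camera manager that applies camera settings widget controls to the player pawn's CineCamera.
; BeginPlay caches the widget and pawn, binds depth-of-field and auto-exposure toggles, and starts with auto exposure on.
; Toggles swap focus settings between tracking and disabled, or exposure between histogram and manual metering.
; Tick applies the widget's focal length and either writes exposure compensation back to the widget in auto or applies its bias in manual.
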(event Custom|SetAutoExposureOn
  ;[1 1 1] InitCamera
  (Variables|Default|SetAutoExposure true)
  (Variables|/Script/Engine.CameraComponent|SetPostProcessSettings (Variables|/Game/Blueprint/BP_MyPawn.BP_MyPawn_C|GetCineCamera (Variables|Default|GetAs%20BP%20My%20Pawn)) (Utilities|Struct|MakePostProcessSettings "AEM_Histogram" 13.0 17.0)))

(event Custom|SetAutoExposureOff
  ;[1 1 1] InitCamera
  (Variables|Default|SetAutoExposure false)
  (Variables|/Script/Engine.CameraComponent|SetPostProcessSettings (Variables|/Game/Blueprint/BP_MyPawn.BP_MyPawn_C|GetCineCamera (Variables|Default|GetAs%20BP%20My%20Pawn)) (Utilities|Struct|MakePostProcessSettings "AEM_Manual")))

(event Custom|InitCamera
  (bind _aswbp_camera_setting (Variables|Default|GetAsWBP%20Camera%20Setting))
  ;[1 1 1] InitCamera
  (EventDispatchers|BindEventtoDepthOfFieldon _aswbp_camera_setting (delegate Custom|SetDepthOfFieldOn))
  (EventDispatchers|BindEventtoDepthOfFieldOff _aswbp_camera_setting (delegate Custom|SetDepthOfFieldOff))
  (EventDispatchers|BindEventtoAutoExposureon _aswbp_camera_setting (delegate Custom|SetAutoExposureOn))
  (EventDispatchers|BindEventtoAutoExposureOff _aswbp_camera_setting (delegate Custom|SetAutoExposureOff)))

(event Custom|SetDepthOfFieldOn
  ;[1 1 1] InitCamera
  (Variables|/Script/CinematicCamera.CineCameraComponent|SetFocusSettings (Variables|/Game/Blueprint/BP_MyPawn.BP_MyPawn_C|GetCineCamera (Variables|Default|GetAs%20BP%20My%20Pawn)) (Variables|Default|GetFocusSettingTracking)))

(event Custom|SetDepthOfFieldOff
  ;[1 1 1] InitCamera
  (Variables|/Script/CinematicCamera.CineCameraComponent|SetFocusSettings (Variables|/Game/Blueprint/BP_MyPawn.BP_MyPawn_C|GetCineCamera (Variables|Default|GetAs%20BP%20My%20Pawn)) (Variables|Default|GetFocusSettingDisable)))

(event EventBeginPlay
  (Utilities|FlowControl|Sequence
    (:then_0
      ;[1 1 1] InitWBP
      (bind _returnvalue (Actor|GetActorOfClass "/Game/Blueprint/Manager/BPM_Widget.BPM_Widget_C"))
      (Variables|Default|SetAsWBP%20Camera%20Setting (Variables|/Game/Blueprint/Widget/WBP_Widgets.WBP_Widgets_C|GetWBP_CameraSetting (Variables|/Game/Blueprint/Manager/BPM_Widget.BPM_Widget_C|GetAsWBP_Widget _returnvalue))))
    (:then_1
      ;[1 1 1] InitPawn
      (bind _asbp_my_pawn (Utilities|Casting|CastToBP_MyPawn (Game|Player|GetPlayerPawn 0)))
      (Variables|Default|SetAs%20BP%20My%20Pawn _asbp_my_pawn))
    (:then_2
      (CallFunction|InitCamera)
      (CallFunction|SetAutoExposureon))))

(event Collision|EventActorBeginOverlap
  (params (OtherActor :type Actor%20Object%20Reference)))

(event EventTick
  (params (DeltaSeconds :type Float%20%28single-precision%29))
  ;[1 1 1] CameraSetting
  (bind _value (Default|FNCGetValueCurrentFocusLength (Variables|Default|GetAsWBP%20Camera%20Setting)))
  (Variables|/Script/CinematicCamera.CineCameraComponent|SetCurrentFocalLength (Variables|/Game/Blueprint/BP_MyPawn.BP_MyPawn_C|GetCineCamera (Variables|Default|GetAs%20BP%20My%20Pawn)) _value)
  (if (Variables|Default|GetAutoExposure)
    (Default|FNCSetValueAutoExposureBias (Variables|Default|GetAsWBP%20Camera%20Setting) (Utilities|Struct|BreakPostProcessSettings (Variables|/Script/Engine.CameraComponent|GetPostProcessSettings (Variables|/Game/Blueprint/BP_MyPawn.BP_MyPawn_C|GetCineCamera (Variables|Default|GetAs%20BP%20My%20Pawn)))))
    (else
      (bind _value_2 (Default|FNCGetValueAutoExposureBias (Variables|Default|GetAsWBP%20Camera%20Setting)))
      (Variables|/Script/Engine.CameraComponent|SetPostProcessSettings (Variables|/Game/Blueprint/BP_MyPawn.BP_MyPawn_C|GetCineCamera (Variables|Default|GetAs%20BP%20My%20Pawn)) (Utilities|Struct|MakePostProcessSettings _value_2)))))

(fn ConstructionScript)