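; Screen manager that controls the visibility and surface material of the BP_Screen actor in the level.
; On BeginPlay it finds the screen setting widget via BPM_Widget and the BP_Screen actor, then applies a default white material to both screen meshes.
; It binds the widget's events to handlers that hide or show the screen or swap both meshes to preset materials such as tiles, wood, stone, fabric and granite.
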(event Custom|SetScreenMatMetallicBlack
  ;[1 1 1] Init Bind
  (Rendering|Material|SetMaterial (Variables|/Game/Blueprint/Actor/BP_Screen.BP_Screen_C|GetScreen (Variables|Default|GetAsBP_Screen)) 0 "/Game/Material/M_MetallicBlack.M_MetallicBlack"))

(event Custom|SetScreenMatWoodFloor
  ;[1 1 1] Init Bind
  (Rendering|Material|SetMaterial (Variables|/Game/Blueprint/Actor/BP_Screen.BP_Screen_C|GetScreen (Variables|Default|GetAsBP_Screen)) 0 "/Game/Material/MI_WoodenFloor.MI_WoodenFloor"))

(event Custom|SetScreenMatStoneWall
  ;[1 1 1] Init Bind
  (Rendering|Material|SetMaterial (Variables|/Game/Blueprint/Actor/BP_Screen.BP_Screen_C|GetScreen (Variables|Default|GetAsBP_Screen)) 0 "/Game/Material/MI_Stone_Wall_vlswfjc_2K.MI_Stone_Wall_vlswfjc_2K"))

(event Custom|SetScreenMatGypsum
  ;[1 1 1] Init Bind
  (Rendering|Material|SetMaterial (Variables|/Game/Blueprint/Actor/BP_Screen.BP_Screen_C|GetScreen (Variables|Default|GetAsBP_Screen)) 0 "/Game/Material/MI_Gypsum_Tiles_uldnbcdn_2K.MI_Gypsum_Tiles_uldnbcdn_2K"))

(event Custom|SetScreenMatWoodenPlankWall
  ;[1 1 1] Init Bind
  (Rendering|Material|SetMaterial (Variables|/Game/Blueprint/Actor/BP_Screen.BP_Screen_C|GetScreen (Variables|Default|GetAsBP_Screen)) 0 "/Game/Material/MI_Wooden_Planks_Wall_vmchejun_2K.MI_Wooden_Planks_Wall_vmchejun_2K"))

(event Custom|SetScreenMatDarkGreyFabric
  ;[1 1 1] Init Bind
  (Rendering|Material|SetMaterial (Variables|/Game/Blueprint/Actor/BP_Screen.BP_Screen_C|GetScreen (Variables|Default|GetAsBP_Screen)) 0 "/Game/Material/MI_Dark_Grey_Fabric_sbkla2p0_2K.MI_Dark_Grey_Fabric_sbkla2p0_2K"))

(event Custom|SetScreenMatViaLatteaGranite
  ;[1 1 1] Init Bind
  (Rendering|Material|SetMaterial (Variables|/Game/Blueprint/Actor/BP_Screen.BP_Screen_C|GetScreen (Variables|Default|GetAsBP_Screen)) 0 "/Game/Material/MI_Via_Lattea_Granite_weoldhcv_2K.MI_Via_Lattea_Granite_weoldhcv_2K"))

(event Custom|HideScreen
  ;[1 1 1] Init Bind
  (Rendering|SetActorHiddenInGame (Variables|Default|GetAsBP_Screen) true))

(event Custom|ShowScreen
  ;[1 1 1] Init Bind
  (Rendering|SetActorHiddenInGame (Variables|Default|GetAsBP_Screen) false))

(event Custom|SetScreenMatDefaultWhite
  ;[1 1 1] Init Bind
  (Rendering|Material|SetMaterial (Variables|/Game/Blueprint/Actor/BP_Screen.BP_Screen_C|GetScreen (Variables|Default|GetAsBP_Screen)) 0 "/Game/Material/M_DefaultWhite.M_DefaultWhite"))

(event Custom|SetScreenMatDefaultBlack
  ;[1 1 1] Init Bind
  (Rendering|Material|SetMaterial (Variables|/Game/Blueprint/Actor/BP_Screen.BP_Screen_C|GetScreen (Variables|Default|GetAsBP_Screen)) 0 "/Game/Material/M_DefaultBlack.M_DefaultBlack"))

(event Custom|SetScreenMatCeramicTiles
  ;[1 1 1] Init Bind
  (Rendering|Material|SetMaterial (Variables|/Game/Blueprint/Actor/BP_Screen.BP_Screen_C|GetScreen (Variables|Default|GetAsBP_Screen)) 0 "/Game/Material/MI_Patterened_Ceramic_Tiles_uk0ocizfw_2K.MI_Patterened_Ceramic_Tiles_uk0ocizfw_2K"))

(event EventBeginPlay
  (Utilities|FlowControl|Sequence
    (:then_0
      ;[1 1 1] Init WBP
      (bind _returnvalue (Actor|GetActorOfClass "/Game/Blueprint/Manager/BPM_Widget.BPM_Widget_C"))
      (Variables|Default|SetAsWBP_ScreenSetting (Variables|/Game/Blueprint/Widget/WBP_Widgets.WBP_Widgets_C|GetWBP_ScreenSetting (Variables|/Game/Blueprint/Manager/BPM_Widget.BPM_Widget_C|GetAsWBP_Widget _returnvalue))))
    (:then_1
      ;[1 1 1] Init Material
      (bind _returnvalue_2 (Actor|GetActorOfClass "/Game/Blueprint/Actor/BP_Screen.BP_Screen_C"))
      (bind _output_get (Variables|Default|SetAsBP_Screen _returnvalue_2))
      (Rendering|Material|SetMaterial (Variables|/Game/Blueprint/Actor/BP_Screen.BP_Screen_C|GetScreen _output_get) 0 "/Game/Material/M_DefaultWhite.M_DefaultWhite"))
    (:then_2
      ;[1 1 1] Init Bind
      (EventDispatchers|BindEventtoHideScreen (Variables|Default|GetAsWBP_ScreenSetting) (delegate Custom|HideScreen))
      (EventDispatchers|BindEventtoShowScreen (Variables|Default|GetAsWBP_ScreenSetting) (delegate Custom|ShowScreen))
      (EventDispatchers|BindEventtoDefaultWhite (Variables|Default|GetAsWBP_ScreenSetting) (delegate Custom|SetScreenMatDefaultWhite))
      (EventDispatchers|BindEventtoDefaultBlack (Variables|Default|GetAsWBP_ScreenSetting) (delegate Custom|SetScreenMatDefaultBlack))
      (EventDispatchers|BindEventtoCeramicTiles (Variables|Default|GetAsWBP_ScreenSetting) (delegate Custom|SetScreenMatCeramicTiles))
      (EventDispatchers|BindEventtoMetallicBlack (Variables|Default|GetAsWBP_ScreenSetting) (delegate Custom|SetScreenMatMetallicBlack))
      (EventDispatchers|BindEventtoWoodenWall (Variables|Default|GetAsWBP_ScreenSetting) (delegate Custom|SetScreenMatWoodFloor))
      (EventDispatchers|BindEventtoStoneWall (Variables|Default|GetAsWBP_ScreenSetting) (delegate Custom|SetScreenMatStoneWall))
      (EventDispatchers|BindEventtoWoodenPlankWall (Variables|Default|GetAsWBP_ScreenSetting) (delegate Custom|SetScreenMatWoodenPlankWall))
      (EventDispatchers|BindEventtoDarkGreyFabric (Variables|Default|GetAsWBP_ScreenSetting) (delegate Custom|SetScreenMatDarkGreyFabric))
      (EventDispatchers|BindEventtoViaLatteaGranite (Variables|Default|GetAsWBP_ScreenSetting) (delegate Custom|SetScreenMatViaLatteaGranite))
      (EventDispatchers|BindEventtoGypsum (Variables|Default|GetAsWBP_ScreenSetting) (delegate Custom|SetScreenMatGypsum)))))

(fn ConstructionScript)