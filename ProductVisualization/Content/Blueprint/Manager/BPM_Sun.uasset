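; Sun manager actor that lets a sun-height UI widget control the level's SunSky directional light.
; On BeginPlay it gets the widget through BPM_Widget, finds the SunSky, binds the widget's solar-time on/off events and starts with solar time on.
; Those events toggle the light's Atmosphere Sun Light setting.
; Every Tick polls the widget's height value and applies it as the light's pitch.
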(event Custom|SolarTimeOn
  ;[1 1 1] Init Sun Setting
  (Class|DirectionalLightComponent|SetAtmosphereSunLight (Variables|/SunPosition/SunSky.SunSky_C|GetDirectionalLight (Variables|Default|GetAsSunSky)) true))

(event Custom|SolarTimeOff
  ;[1 1 1] Init Sun Setting
  (Class|DirectionalLightComponent|SetAtmosphereSunLight (Variables|/SunPosition/SunSky.SunSky_C|GetDirectionalLight (Variables|Default|GetAsSunSky)) false))

(event Custom|InitSunSetting
  (bind _aswbp_sunhight (Variables|Default|GetAsWBP_SunHight))
  ;[1 1 1] Init Sun Setting
  (Utilities|FlowControl|Sequence
    (:then_0
      (bind _outactors (Actor|GetAllActorsOfClass "/SunPosition/SunSky.SunSky_C"))
      (for _array_element _outactors
        (Variables|Default|SetAsSunSky _array_element)))
    (:then_1
      (EventDispatchers|BindEventtoSolarTimeon _aswbp_sunhight (delegate Custom|SolarTimeOn))
      (EventDispatchers|BindEventtoSolarTimeOff _aswbp_sunhight (delegate Custom|SolarTimeOff)))))

(event EventBeginPlay
  (Utilities|FlowControl|Sequence
    (:then_0
      ;[1 1 1] Init WBP
      (bind _returnvalue (Actor|GetActorOfClass "/Game/Blueprint/Manager/BPM_Widget.BPM_Widget_C"))
      (Variables|Default|SetAsWBP_SunHight (Variables|/Game/Blueprint/Widget/WBP_Widgets.WBP_Widgets_C|GetWBP_SunHight (Variables|/Game/Blueprint/Manager/BPM_Widget.BPM_Widget_C|GetAsWBP_Widget _returnvalue))))
    (:then_1
      (CallFunction|InitSunSetting)
      (CallFunction|SolarTimeon))))

(event Collision|EventActorBeginOverlap
  (params (OtherActor :type Actor%20Object%20Reference)))

(event EventTick
  (params (DeltaSeconds :type Float%20%28single-precision%29))
  (bind _assunsky (Variables|Default|GetAsSunSky))
  (bind _directionallight (Variables|/SunPosition/SunSky.SunSky_C|GetDirectionalLight _assunsky))
  ;[1 1 1] Set Sun Hight
  (bind _value (Default|FNCGetValueSunHight (Variables|Default|GetAsWBP_SunHight)))
  (Transformation|SetWorldRotation _directionallight (Math|Rotator|MakeRotator (.roll (Transformation|GetWorldRotation _directionallight)) _value 0.0) false false))

(fn ConstructionScript)